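; Player 2 character Blueprint that feeds head orientation to toon materials through the MPC_Char_Toon parameter collection.
; Every Tick it reads the world-space head bone transform from MECharPlayer2 and writes its up, right and forward vectors to HeadUp, HeadRight and HeadForward.
; Because a parameter collection is global, every material sampling it receives this one character's head axes.
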(event `self.ReceiveTick`
  (params (DeltaSeconds :type "Float (single-precision)"))
  (bind _rotation (.rotation (`SkinnedMeshComponent.GetBoneTransform` (`self.ME_Char_Player2`) "head" "RTS_World")))
  (`KismetMaterialLibrary.SetVectorParameterValue` "/Game/Characters/Materials/MPC_Char_Toon.MPC_Char_Toon" "HeadUp" (`KismetMathLibrary.Conv_VectorToLinearColor` (`KismetMathLibrary.GetUpVector` _rotation)))
  (`KismetMaterialLibrary.SetVectorParameterValue` "/Game/Characters/Materials/MPC_Char_Toon.MPC_Char_Toon" "HeadRight" (`KismetMathLibrary.Conv_VectorToLinearColor` (`KismetMathLibrary.GetRightVector` _rotation)))
  (`KismetMaterialLibrary.SetVectorParameterValue` "/Game/Characters/Materials/MPC_Char_Toon.MPC_Char_Toon" "HeadForward" (`KismetMathLibrary.Conv_VectorToLinearColor` (`KismetMathLibrary.GetForwardVector` _rotation))))

(fn `UserConstructionScript`)