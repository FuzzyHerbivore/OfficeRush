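; BP_CableVent is an environment prop that strings hanging cables from its root mesh to a referenced TargetCables actor.
; The construction script destroys existing cable components, then calls AddCables, which pairs both meshes' sockets by index up to the smaller count.
; Each pair gets a cable with randomised slack, width and material, plus connector meshes at both ends.
; The target-end mesh attaches to its socket on the other actor, snapping to its rotation.
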(fn `AddCables`
  (bind _returnvalue (`SceneComponent.GetAllSocketNames` (`self.RootMesh`)))
  (bind _rootcomponent (`Actor.RootComponent` (`self.TargetCables`)))
  (bind _returnvalue_2 (`SceneComponent.GetAllSocketNames` _rootcomponent))
  (`/Engine/EditorBlueprintResources/StandardMacros.IsValid` (`self.TargetCables`)
    (:`Is Valid`
      (for _index (range (`KismetMathLibrary.Min` (`KismetArrayLibrary.Array_Length` _returnvalue) (`KismetArrayLibrary.Array_Length` _returnvalue_2)))
        (bind _returnvalue_3 (`AddComponent|NODE_AddCableComponent-0`))
        (bind _output_get (set `self.CableComponent` _returnvalue_3))
        (bind _returnvalue_4 (`SceneComponent.GetSocketLocation` (`self.RootMesh`) (`|GetArrayItem` _returnvalue _index)))
        (`SceneComponent.K2_SetWorldLocation` _output_get _returnvalue_4 false false)
        (bind _output (`|GetArrayItem` _returnvalue_2 _index))
        (bind _returnvalue_5 (`SceneComponent.GetSocketLocation` _rootcomponent _output))
        (set `CableComponent.EndLocation` (`KismetMathLibrary.InverseTransformLocation` (`SceneComponent.K2_GetComponentToWorld` (`self.RootMesh`)) _returnvalue_5) (`self.CableComponent`))
        (set `CableComponent.CableLength` (* (`KismetMathLibrary.VSize` (- _returnvalue_4 _returnvalue_5)) (`KismetMathLibrary.RandomFloatInRange` (`self.MinCableLength`) (`self.MaxCableLength`))) (`self.CableComponent`))
        (set `CableComponent.CableWidth` (`KismetMathLibrary.RandomFloatInRange` (`self.MinCableWidth`) (`self.MaxCableWidth`)) (`self.CableComponent`))
        (`PrimitiveComponent.SetMaterial` (`self.CableComponent`) 0 (`KismetArrayLibrary.Array_Random` (`self.MaterialRandomiser`)))
        (bind _returnvalue_6 (`AddComponent|NODE_AddStaticMeshComponent-0`))
        (`StaticMeshComponent.SetStaticMesh` _returnvalue_6 (`self.OutputMeshBase`))
        (`SceneComponent.K2_SetWorldLocation` _returnvalue_6 _returnvalue_4 false false)
        (bind _returnvalue_7 (`AddComponent|NODE_AddStaticMeshComponent-1`))
        (`StaticMeshComponent.SetStaticMesh` _returnvalue_7 (`self.OutputMeshTarget`))
        (`SceneComponent.K2_AttachToComponent` _returnvalue_7 (`Actor.RootComponent` (`self.TargetCables`)) _output "KeepWorld" "SnapToTarget" "KeepWorld" false)
        (`SceneComponent.K2_SetWorldLocation` _returnvalue_7 _returnvalue_5 false false)))))

(fn `UserConstructionScript`
  (`|ExecutionSequence`
    (:`then_0`
      (for _array_element (`self.K2_GetComponentsByClass` "/Script/CableComponent.CableComponent")
        (`ActorComponent.K2_DestroyComponent` _array_element)))
    (:`then_1`
      (`self.AddCables`))))