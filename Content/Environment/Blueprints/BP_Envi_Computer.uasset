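; Environment computer prop that procedurally strings cables from its mesh sockets to the sockets on a Target actor's root component.
; The construction script destroys existing cable components, then runs SpawnCables, which pairs both socket lists by index up to the shorter count.
; Each pair gets a cable with randomized length and width, plus a static mesh at each end, attached to the computer and Target respectively.
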(fn `SpawnCables`
  (bind _returnvalue (`SceneComponent.GetAllSocketNames` (`self.SM_Computer`)))
  (bind _rootcomponent (`Actor.RootComponent` (`self.Target`)))
  (bind _returnvalue_2 (`SceneComponent.GetAllSocketNames` _rootcomponent))
  (`/Engine/EditorBlueprintResources/StandardMacros.IsValid` (`self.Target`)
    (:`Is Valid`
      (for _index (range (`KismetMathLibrary.Min` (`KismetArrayLibrary.Array_Length` _returnvalue) (`KismetArrayLibrary.Array_Length` _returnvalue_2)))
        (bind _returnvalue_3 (`AddComponent|NODE_AddCableComponent-0`))
        (bind _output_get (set `self.CableComponent` _returnvalue_3))
        (set `CableComponent.CollisionFriction` (`self.Collision Friction`) _output_get)
        (bind _returnvalue_4 (`SceneComponent.GetSocketLocation` (`self.SM_Computer`) (`|GetArrayItem` _returnvalue _index)))
        (`SceneComponent.K2_SetWorldLocation` (`self.CableComponent`) _returnvalue_4 false false)
        (bind _output (`|GetArrayItem` _returnvalue_2 _index))
        (bind _returnvalue_5 (`SceneComponent.GetSocketLocation` _rootcomponent _output))
        (set `CableComponent.EndLocation` (`KismetMathLibrary.InverseTransformLocation` (`SceneComponent.K2_GetComponentToWorld` (`self.SM_Computer`)) _returnvalue_5) (`self.CableComponent`))
        (set `CableComponent.CableLength` (* (`KismetMathLibrary.VSize` (- _returnvalue_4 _returnvalue_5)) (`KismetMathLibrary.RandomFloatInRange` (`self.Minimum Cable Length Multiplier`) (`self.Maximum cable Length Multiplier`))) (`self.CableComponent`))
        (set `CableComponent.CableWidth` (`KismetMathLibrary.RandomFloatInRange` (`self.MinimumCableWidth`) (`self.Maximum CableWidth`)) (`self.CableComponent`))
        (bind _returnvalue_6 (`AddComponent|NODE_AddStaticMeshComponent-0`))
        (`SceneComponent.K2_AttachToComponent` _returnvalue_6 (`self.SM_Computer`) "None" "KeepWorld" "SnapToTarget" "KeepWorld" false)
        (`SceneComponent.K2_SetWorldLocation` _returnvalue_6 _returnvalue_4 false false)
        (bind _returnvalue_7 (`AddComponent|NODE_AddStaticMeshComponent-1`))
        (`SceneComponent.K2_AttachToComponent` _returnvalue_7 (`Actor.RootComponent` (`self.Target`)) _output "KeepWorld" "SnapToTarget" "KeepWorld" false)
        (`SceneComponent.K2_SetWorldLocation` _returnvalue_7 _returnvalue_5 false false)))))

(fn `UserConstructionScript`
  (`|ExecutionSequence`
    (:`then_0`
      (for _array_element (`self.K2_GetComponentsByClass` "/Script/CableComponent.CableComponent")
        (`ActorComponent.K2_DestroyComponent` _array_element)))
    (:`then_1`
      (`self.SpawnCables`))))