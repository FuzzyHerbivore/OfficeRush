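; BP_PCG_Cables_01 is an environment actor that strings cables from its static mesh to a Target actor.
; Its construction script applies the mesh, then pairs sockets with those on the Target's root component by index, up to the smaller count.
; Each pair gets a new Cable component, with length set to socket distance times an unseeded random multiplier, so slack varies whenever construction reruns.
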(event EventBeginPlay)

(event Collision|EventActorBeginOverlap
  (params (OtherActor :type Actor%20Object%20Reference)))

(event EventTick
  (params (DeltaSeconds :type Float%20%28single-precision%29)))

(fn ConstructionScript
  (bind _sm_rootactor (Variables|Default|GetSM_RootActor))
  (bind _target (Variables|Default|GetTarget))
  (bind _returnvalue (Transformation|GetAllSocketNames _sm_rootactor))
  (bind _rootcomponent (Variables|/Script/Engine.Actor|GetRootComponent _target))
  (bind _returnvalue_2 (Transformation|GetAllSocketNames _rootcomponent))
  (Components|StaticMesh|SetStaticMesh (Variables|Default|GetSM_RootActor) (Variables|Default|GetStaticMesh))
  (Utilities|IsValid (Variables|Default|GetTarget)
    (:Is%20Valid
      (for _index (range 0 (- (Math|Integer|Min(Integer) (Utilities|Array|Length _returnvalue) (Utilities|Array|Length _returnvalue_2)) 1))
        (bind _returnvalue_3 (AddComponent|AddCableComponent false))
        (Transformation|SetWorldLocation _returnvalue_3 (Transformation|GetSocketLocation (Variables|Default|GetSM_RootActor) (Utilities|Array|Get(acopy) _returnvalue _index)) false false)
        (Variables|/Script/CableComponent.CableComponent|SetEndLocation _returnvalue_3 (Math|Transform|InverseTransformLocation (Transformation|GetWorldTransform (Variables|Default|GetSM_RootActor)) (Transformation|GetSocketLocation _rootcomponent (Utilities|Array|Get(acopy) _returnvalue_2 _index))))
        (Variables|/Script/CableComponent.CableComponent|SetCableLength _returnvalue_3 (* (Math|Vector|VectorLength (- (Transformation|GetSocketLocation (Variables|Default|GetSM_RootActor) (Utilities|Array|Get(acopy) _returnvalue _index)) (Transformation|GetSocketLocation _rootcomponent (Utilities|Array|Get(acopy) _returnvalue_2 _index)))) (Math|Random|RandomFloatinRange (Variables|Default|GetMinimum%20Cable%20Length%20Multiplier) (Variables|Default|GetMaximum%20cable%20Length%20Multiplier))))))))