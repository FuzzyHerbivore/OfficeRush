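; BP_Door is a keycard-coded forcefield door that opens and closes through Switch or Toggle, where "on" means closed.
; The construction script sets initial visibility and tints a dynamic material and Niagara effect from keycard data tables.
; Opening and closing switch collision immediately, trigger particles and sound, and animate opacity and noise with timelines.
; Getters expose state, color and authorization token; the door itself performs no keycard check.
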(event `self.ReceiveBeginPlay`
  ; Begin
  (`self.SetCollision` (`self.IsInitiallyClosed`)))

(event `OpenDoor`
  (bind _door_material_instance (`self.Door Material Instance`))
  ; Open Door
  (bind _output_get (set `self.IsClosed` false))
  (`self.SetCollision` _output_get)
  (`ActorComponent.Activate` (`self.FXS_DoorOpen`) false)
  (`GameplayStatics.PlaySoundAtLocation` "/Game/SoundAndMusic/SoundEffects/LockAndKeySounds/MS_DoorOpen.MS_DoorOpen" (`self.K2_GetActorLocation`) (struct) 1.0 1.0 0.0 null null null null)
  (bind (_direction _opacity_down _noisestrength) (`Timeline|Timeline_0` :!via `PlayFromStart`)
    (:`Update`
      (`MaterialInstanceDynamic.SetScalarParameterValue` _door_material_instance "Opacity" _opacity_down)
      (`MaterialInstanceDynamic.SetScalarParameterValue` _door_material_instance "Noise Strength" _noisestrength))
    (:`Finished`
      (`SceneComponent.SetVisibility` (`self.ME_Envi_Door`) false false))))

(event `CloseDoor`
  (bind _door_material_instance (`self.Door Material Instance`))
  ; Close Door
  (bind _output_get (set `self.IsClosed` true))
  (`SceneComponent.SetVisibility` (`self.ME_Envi_Door`) _output_get false)
  (`self.SetCollision` _output_get)
  (`ActorComponent.Activate` (`self.FXS_DoorOpen`) false)
  (`GameplayStatics.PlaySoundAtLocation` "/Game/SoundAndMusic/SoundEffects/LockAndKeySounds/MS_DoorLock.MS_DoorLock" (`self.K2_GetActorLocation`) (struct) 1.0 1.0 0.0 null null null null)
  (bind (_direction _opacityup _noisestrength) (`Timeline|Timeline` :!via `PlayFromStart`)
    (:`Update`
      (`MaterialInstanceDynamic.SetScalarParameterValue` _door_material_instance "Opacity" _opacityup)
      (`MaterialInstanceDynamic.SetScalarParameterValue` _door_material_instance "Noise Strength" _noisestrength))))

(event `/Game/Libraries/Switching/BPI_Switchable.Toggle`
  ; Toggle
  (`self.Switch` (not (`self.IsClosed`))))

(event `/Game/Libraries/Switching/BPI_Switchable.Switch`
  (params (ShouldBeEnabled :type Boolean))
  ; Switch explicitely to on/off
  (if ShouldBeEnabled
    (`self.CloseDoor`)
    (else
      (`self.OpenDoor`))))

(fn `GetAuthorizationToken`
  (returns (AuthorizationToken :type "/Game/Libraries/Authorization/S_AuthorizationToken Structure"))
  (bind _returnvalue (`|GetDataTableRow` "/Game/Libraries/Authorization/DT_AuthorizationTokens.DT_AuthorizationTokens" (`.RowName` (break `DataTableRowHandle` (`.AuthorizationTokensRow_31_5D9163E944FAC1CD1D4C2886CBDD2036` (break `/Game/Features/Doors/S_KeycardData` (`self.AuthorizedKeycardData`))))))
    (:`then`
      (return _returnvalue))))

(fn `GetColorCurveValue`
  (returns (ColorCurveValue :type "Float (double-precision)"))
  (bind _returnvalue (`|GetDataTableRow` "/Game/Features/Doors/DT_KeycardColors.DT_KeycardColors" (`.RowName` (break `DataTableRowHandle` (`.KeycardColorsRow_41_12EE567C4040F331F305538E9C89AD01` (break `/Game/Features/Doors/S_KeycardData` (`self.AuthorizedKeycardData`))))))
    (:`then`
      (return (break `/Game/Features/Doors/S_KeycardColor` _returnvalue)))))

(fn `GetIsSwitchedOn`
  (returns (IsSwitchedOn :type Boolean))
  (return (`self.IsClosed`)))

(fn `SetCollision`
  (params (IsOn :type Boolean))
  (bind _me_envi_door (`self.ME_Envi_Door`))
  (if IsOn
    (`PrimitiveComponent.SetCollisionEnabled` _me_envi_door "QueryAndProbe")
    (else
      (`PrimitiveComponent.SetCollisionEnabled` _me_envi_door "NoCollision"))))

(fn `UserConstructionScript`
  (bind (_authorizedkeycardrow_datatable _authorizedkeycardrow_rowname) (break `DataTableRowHandle` (`self.AuthorizedKeycardRow`)))
  (bind _output_get (set `self.IsClosed` (`self.IsInitiallyClosed`)))
  (`SceneComponent.SetVisibility` (`self.ME_Envi_Door`) _output_get false)
  (bind _returnvalue (`|GetDataTableRow` "/Game/Features/Doors/DT_Keycards.DT_Keycards" _authorizedkeycardrow_rowname)
    (:`then`
      (bind _output_get_2 (set `self.AuthorizedKeycardData` _returnvalue))
      (bind _returnvalue_2 (`|GetDataTableRow` "/Game/Features/Doors/DT_KeycardColors.DT_KeycardColors" (`.RowName` (break `DataTableRowHandle` (`.KeycardColorsRow_41_12EE567C4040F331F305538E9C89AD01` (break `/Game/Features/Doors/S_KeycardData` _output_get_2)))))
        (:`then`
          (bind _returnvalue_3 (`PrimitiveComponent.CreateDynamicMaterialInstance` (`self.ME_Envi_Door`) 0 "/Game/Vfx/Materials/M_VFX_Forcefield_02_Yellow.M_VFX_Forcefield_02_Yellow" "None"))
          (bind _output_get_3 (set `self.Door Material Instance` _returnvalue_3))
          (`MaterialInstanceDynamic.SetScalarParameterValue` _output_get_3 "BaseColor LUT" (break `/Game/Features/Doors/S_KeycardColor` _returnvalue_2))
          (`NiagaraComponent.SetNiagaraVariableFloat` (`self.FXS_DoorOpen`) "User_ParticleColor" (break `/Game/Features/Doors/S_KeycardColor` _returnvalue_2)))))))