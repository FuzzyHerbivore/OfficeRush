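; BP_Keycard is a collectable keycard that interactors with an inventory can pick up, supplying an authorization token, name, icon and category.
; Data tables define each card, with construction tinting its dynamic material and Niagara effects through color LUT values.
; Focus toggles selection particles and a timeline hover lerp.
; Collection hides the mesh and disables collision; dropping re-enables it at the given location, while reset restores its spawn position, delayed unless the game restarted.
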(event `self.ReceiveBeginPlay`
  ; Begin
  (`ActorComponent.Deactivate` (`self.FXS_VFX_Selection_01`)))

(event `/Game/Libraries/Inventory/BPI_Collectable.OnCollected`
  ; OnCollected
  (`ActorComponent.Activate` (`self.FXS_VFX_PickUp`) false)
  (`self.Disable`))

(event `/Game/Libraries/Inventory/BPI_Collectable.OnReset`
  ; OnReset
  (if (`self.WasGameRestarted`)
    (set `self.WasGameRestarted` false)
    (else
      (`KismetSystemLibrary.Delay` (`self.RespawnDelay`))))
  (`self.EnableAtLocation` (`self.SpawnPosition`))
  (`ActorComponent.Deactivate` (`self.FXS_VFX_PickUp`)))

(event `OnGameRestartedNotifyKeycard`
  (set `self.WasGameRestarted` true)
  (`self.OnReset`))

(event `/Game/Libraries/Inventory/BPI_Collectable.OnDropped`
  (params (Location :type "Vector Structure"))
  ; OnDropped
  (`self.EnableAtLocation` Location)
  (`ActorComponent.Deactivate` (`self.FXS_VFX_PickUp`)))

(event `/Game/Libraries/Interaction/BPI_Interactable.Interact`
  (params (Interactor :type "Actor Object Reference (by ref)"))
  ; Interact
  (bind _asbpi_inventory (cast `/Game/Libraries/Inventory/BPI_Inventory` Interactor))
  (bind _asbpi_collectable (cast `/Game/Libraries/Inventory/BPI_Collectable` self))
  (bind _wassuccessful (`/Game/Libraries/Inventory/BPI_Inventory.Collect` _asbpi_inventory _asbpi_collectable))
  (if _wassuccessful
    (`/Game/Libraries/Inventory/BPI_Collectable.OnCollected` _asbpi_collectable)
    (`GameplayStatics.PlaySoundAtLocation` "/Game/SoundAndMusic/SoundEffects/InteractionSounds/MS_PickUp.MS_PickUp" (`self.K2_GetActorLocation`) (struct) 1.0 1.0 0.0 null null null null)))

(event `/Game/Libraries/Interaction/BPI_Interactable.Focus`
  (params (IsOn :type Boolean))
  ; Focus
  (if (not (== IsOn (`self.IsFocused`)))
    (bind _output_get (set `self.IsFocused` IsOn))
    (if _output_get
      (`ActorComponent.Activate` (`self.FXS_VFX_Selection_01`) false)
      (bind (_direction _hover_animation) (`Timeline|Timeline` :!via `PlayFromStart`)
        (:`Update`
          (`MaterialInstanceDynamic.SetScalarParameterValue` (`self.DynamicMaterialInstance`) "HoverLerp" _hover_animation)))
      (else
        (`ActorComponent.Deactivate` (`self.FXS_VFX_Selection_01`))
        (bind (_direction_2 _hover_animation_2) (`Timeline|Timeline_0` :!via `ReverseFromEnd`)
          (:`Update`
            (`MaterialInstanceDynamic.SetScalarParameterValue` (`self.DynamicMaterialInstance`) "HoverLerp" _hover_animation_2)))))))

(fn `Disable`
  (bind _sm_keycard (`self.SM_Keycard`))
  (`SceneComponent.SetVisibility` _sm_keycard false false)
  (`PrimitiveComponent.SetCollisionEnabled` _sm_keycard "NoCollision"))

(fn `EnableAtLocation`
  (params (Location :type "Vector Structure"))
  (bind _sm_keycard (`self.SM_Keycard`))
  (`self.K2_SetActorLocation` self Location false true)
  (`SceneComponent.SetVisibility` _sm_keycard true false)
  (`PrimitiveComponent.SetCollisionEnabled` _sm_keycard "QueryAndPhysics"))

(fn `GetActor`
  (returns (Actor :type "Actor Object Reference"))
  (return self))

(fn `GetAuthorizationToken`
  (returns (AuthorizationToken :type "/Game/Libraries/Authorization/S_AuthorizationToken Structure"))
  (bind (_keycarddata_name _keycarddata_symboltextureemission _keycarddata_keycardcolorsrow _keycarddata_uiicon _keycarddata_authorizationtokensrow) (break `/Game/Features/Doors/S_KeycardData` (`self.KeycardData`)))
  (bind _returnvalue (`|GetDataTableRow` "/Game/Libraries/Authorization/DT_AuthorizationTokens.DT_AuthorizationTokens" (`.RowName` (break `DataTableRowHandle` _keycarddata_authorizationtokensrow)))
    (:`then`
      (return _returnvalue))))

(fn `GetCollactableIcon`
  (returns (Icon :type "SlateBrushAsset Object Reference"))
  (bind (_keycarddata_name _keycarddata_symboltextureemission _keycarddata_keycardcolorsrow _keycarddata_uiicon) (break `/Game/Features/Doors/S_KeycardData` (`self.KeycardData`)))
  (return _keycarddata_uiicon))

(fn `GetCollectableCategory`
  (returns (Category :type String))
  (bind (_keycarddata_name _keycarddata_symboltextureemission _keycarddata_keycardcolorsrow _keycarddata_uiicon _keycarddata_authorizationtokensrow _keycarddata_collectablecategory) (break `/Game/Features/Doors/S_KeycardData` (`self.KeycardData`)))
  (return _keycarddata_collectablecategory))

(fn `GetCollectableColor`
  (returns (ColorCurveValue :type "Float (double-precision)"))
  (bind (_keycarddata_name _keycarddata_symboltextureemission _keycarddata_keycardcolorsrow) (break `/Game/Features/Doors/S_KeycardData` (`self.KeycardData`)))
  (bind _returnvalue (`|GetDataTableRow` "/Game/Features/Doors/DT_KeycardColors.DT_KeycardColors" (`.RowName` (break `DataTableRowHandle` _keycarddata_keycardcolorsrow)))
    (:`then`
      (return (`.ColorCurveValue_11_4CF4C150455F8439D75BACBDDC446605` (break `/Game/Features/Doors/S_KeycardColor` _returnvalue))))))

(fn `GetCollectableName`
  (returns (Name :type String))
  (bind _keycarddata_name (break `/Game/Features/Doors/S_KeycardData` (`self.KeycardData`)))
  (return _keycarddata_name))

(fn `GetCollectionBehavior`
  (returns (CollectionBehavior :type "/Game/Libraries/Inventory/E_CollectionBehavior Enum"))
  (bind (_keycarddata_name _keycarddata_symboltextureemission _keycarddata_keycardcolorsrow _keycarddata_uiicon _keycarddata_authorizationtokensrow _keycarddata_collectablecategory _keycarddata_collectionbehavior) (break `/Game/Features/Doors/S_KeycardData` (`self.KeycardData`)))
  (return _keycarddata_collectionbehavior))

(fn `UserConstructionScript`
  (bind (_keycarddatarow_datatable _keycarddatarow_rowname) (break `DataTableRowHandle` (`self.KeycardDataRow`)))
  (set `self.SpawnPosition` (`self.K2_GetActorLocation` self))
  (bind _returnvalue (`|GetDataTableRow` "/Game/Features/Doors/DT_Keycards.DT_Keycards" _keycarddatarow_rowname)
    (:`then`
      (bind _output_get (set `self.KeycardData` _returnvalue))
      (bind _colorcurvevalue (`self.GetCollectableColor`))
      (bind _returnvalue_2 (`PrimitiveComponent.CreateDynamicMaterialInstance` (`self.SM_Keycard`) 0 "/Game/Environment/Assets/KeyCard/M_Inst_Keycard_Base.M_Inst_Keycard_Base" "None"))
      (bind _output_get_2 (set `self.DynamicMaterialInstance` _returnvalue_2))
      (`MaterialInstanceDynamic.SetScalarParameterValue` _output_get_2 "TintColor LUT" _colorcurvevalue)
      (`MaterialInstanceDynamic.SetScalarParameterValue` (`self.DynamicMaterialInstance`) "EmissiveColor LUT" _colorcurvevalue)
      (`NiagaraComponent.SetNiagaraVariableFloat` (`self.FXS_VFX_Selection_01`) "User_ParticleColor" _colorcurvevalue)
      (`NiagaraComponent.SetVariableFloat` (`self.FXS_VFX_PickUp`) "User_ParticleColor" _colorcurvevalue)
      (`MaterialInstanceDynamic.SetTextureParameterValue` (`self.DynamicMaterialInstance`) "Emissive Mask" (`.SymbolTextureEmission_55_075D23A0424CA58F1A387A9A79A08A52` (break `/Game/Features/Doors/S_KeycardData` _output_get))))))