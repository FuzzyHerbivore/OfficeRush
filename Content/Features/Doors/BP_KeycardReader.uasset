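; Keycard reader actor that toggles its linked Door when an interactor is authorized for that door's token.
; Interact checks the interactor against the token, notifies the player controller of correct or wrong use, and plays a fail sound on refusal.
; The construction script tints the reader material and selection particles from the Door's color curve value.
; Focus toggles those particles and animates a hover material lerp, while a door event keeps its cached state updated.
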(event `self.ReceiveBeginPlay`
  (add `/Game/Features/Doors/BP_Door.SwitchStateUpdated` (`self.Door`) (delegate `SwitchStateUpdated`)))

(event `SwitchStateUpdated`
  (params (IsSwitchedOn :type Boolean))
  (bind _asbpi_switchable (cast `/Game/Libraries/Switching/BPI_Switchable` (`self.Door`)))
  (bind _isswitchedon (`/Game/Libraries/Switching/BPI_Switchable.GetIsSwitchedOn` _asbpi_switchable))
  (set `self.IsConnectedDoorClosed` _isswitchedon))

(event `/Game/Libraries/Interaction/BPI_Interactable.Interact`
  (params (Interactor :type "Actor Object Reference (by ref)"))
  (`/Engine/EditorBlueprintResources/StandardMacros.IsValid` Interactor
    (:`Is Valid`
      (bind _asbpi_authorization_token_provider (cast `/Game/Libraries/Authorization/BPI_AuthorizationTokenProvider` (`self.Door`)))
      (bind _authorizationtoken (`/Game/Libraries/Authorization/BPI_AuthorizationTokenProvider.GetAuthorizationToken` _asbpi_authorization_token_provider))
      (bind _asbpi_authorizer (cast `/Game/Libraries/Authorization/BPI_Authorizer` Interactor))
      (bind _isauthorized (`/Game/Libraries/Authorization/BPI_Authorizer.CheckAuthorization` _asbpi_authorizer (`|MakeArray` _authorizationtoken)))
      (bind _aspawn (cast `Pawn` Interactor))
      (bind _asbp_player_controller (cast `/Game/Players/BP_PlayerController` (`Pawn.GetController` _aspawn)))
      (if _isauthorized
        (bind _returnvalue (`GameplayStatics.GetPlayerControllerID` _asbp_player_controller))
        (`/Game/Players/BP_PlayerController.OnPlayerUsedKeycardCorrectlyOnce` _asbp_player_controller _returnvalue)
        (`self.Toggle Switchable Actor`)
        (else
          (`/Game/Players/BP_PlayerController.OnPlayerUsedKeycardWrongOnce` _asbp_player_controller _returnvalue)
          (`GameplayStatics.PlaySoundAtLocation` "/Game/SoundAndMusic/SoundEffects/InteractionSounds/SFX_48_InteractionFail.SFX_48_InteractionFail" (`self.K2_GetActorLocation`) (struct) 1.0 1.0 0.0 null null null null))))))

(event `Toggle Switchable Actor`
  (bind _door (`self.Door`))
  (`/Engine/EditorBlueprintResources/StandardMacros.IsValid` _door
    (:`Is Valid`
      (bind _asbpi_switchable (cast `/Game/Libraries/Switching/BPI_Switchable` _door))
      (`/Game/Libraries/Switching/BPI_Switchable.Toggle` _asbpi_switchable))))

(event `/Game/Libraries/Interaction/BPI_Interactable.Focus`
  (params (IsOn :type Boolean))
  (if (not (== IsOn (`self.IsFocused`)))
    (bind _output_get (set `self.IsFocused` IsOn))
    (if _output_get
      (`ActorComponent.Activate` (`self.FXS_VFX_Particles_Selection`) false)
      (bind (_direction _hover_animation) (`Timeline|Lerp to Hover` :!via `PlayFromStart`)
        (:`Update`
          (`MaterialInstanceDynamic.SetScalarParameterValue` (`self.DynamicMaterialInstance`) "HoverLerp" _hover_animation)))
      (else
        (`ActorComponent.Deactivate` (`self.FXS_VFX_Particles_Selection`))
        (bind (_direction_2 _hover_animation_2) (`Timeline|Lerp To Standard` :!via `ReverseFromEnd`)
          (:`Update`
            (`MaterialInstanceDynamic.SetScalarParameterValue` (`self.DynamicMaterialInstance`) "HoverLerp" _hover_animation_2)))))))

(fn `GetActor`
  (returns (Actor :type "Actor Object Reference"))
  (return self))

(fn `UserConstructionScript`
  (bind _colorcurvevalue (`/Game/Features/Doors/BP_Door.GetColorCurveValue` (`self.Door`)))
  (bind _returnvalue (`PrimitiveComponent.CreateDynamicMaterialInstance` (`self.ReaderMesh`) 0 "/Game/Environment/Assets/KeyCardScanner/M_Inst_Keycardscanner_Base.M_Inst_Keycardscanner_Base" "None"))
  (bind _output_get (set `self.DynamicMaterialInstance` _returnvalue))
  (`MaterialInstanceDynamic.SetScalarParameterValue` _output_get "EmissiveColor LUT" _colorcurvevalue)
  (`NiagaraComponent.SetNiagaraVariableFloat` (`self.FXS_VFX_Particles_Selection`) "User_ParticleColor" _colorcurvevalue))