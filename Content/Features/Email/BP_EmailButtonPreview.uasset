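; Preview actor for the email minigame that displays an arrow button on a plane mesh.
; SetRandomGroup picks one of four directional button groups at random.
; SelectButtonTexture switches on that group, creates a dynamic instance of the mail game arrow material and applies the matching texture as both diffuse and emissive mask.
; The event graph and construction script are empty, so neither function is called within this Blueprint.
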(event `self.ReceiveBeginPlay`)

(fn `SelectButtonTexture`
  (bind _buttondowngfx (`self.ButtonDownGFX`))
  (bind _buttonleftgfx (`self.ButtonLeftGFX`))
  (bind _buttonrightgfx (`self.ButtonRightGFX`))
  (bind _buttonupgfx (`self.ButtonUpGFX`))
  (switch `/Game/Libraries/Minigames/E_EmailButtonGroup` (`self.ButtonGroup`)
    (:`NewEnumerator0`
      (bind _returnvalue (`PrimitiveComponent.CreateDynamicMaterialInstance` (`self.Plane`) 0 "/Game/Environment/Assets/Monitor/M_Inst_MailGameArrows.M_Inst_MailGameArrows" "None"))
      (bind _output_get (set `self.ArrowDMI` _returnvalue))
      (`MaterialInstanceDynamic.SetTextureParameterValue` _output_get "Diffuse" _buttonupgfx)
      (`MaterialInstanceDynamic.SetTextureParameterValue` _output_get "Emissive Mask" _buttonupgfx))
    (:`NewEnumerator1`
      (bind _returnvalue_2 (`PrimitiveComponent.CreateDynamicMaterialInstance` (`self.Plane`) 0 "/Game/Environment/Assets/Monitor/M_Inst_MailGameArrows.M_Inst_MailGameArrows" "None"))
      (bind _output_get_2 (set `self.ArrowDMI` _returnvalue_2))
      (`MaterialInstanceDynamic.SetTextureParameterValue` _output_get_2 "Diffuse" _buttondowngfx)
      (`MaterialInstanceDynamic.SetTextureParameterValue` _output_get_2 "Emissive Mask" _buttondowngfx))
    (:`NewEnumerator2`
      (bind _returnvalue_3 (`PrimitiveComponent.CreateDynamicMaterialInstance` (`self.Plane`) 0 "/Game/Environment/Assets/Monitor/M_Inst_MailGameArrows.M_Inst_MailGameArrows" "None"))
      (bind _output_get_3 (set `self.ArrowDMI` _returnvalue_3))
      (`MaterialInstanceDynamic.SetTextureParameterValue` _output_get_3 "Diffuse" _buttonleftgfx)
      (`MaterialInstanceDynamic.SetTextureParameterValue` _output_get_3 "Emissive Mask" _buttonleftgfx))
    (:`NewEnumerator3`
      (bind _returnvalue_4 (`PrimitiveComponent.CreateDynamicMaterialInstance` (`self.Plane`) 0 "/Game/Environment/Assets/Monitor/M_Inst_MailGameArrows.M_Inst_MailGameArrows" "None"))
      (bind _output_get_4 (set `self.ArrowDMI` _returnvalue_4))
      (`MaterialInstanceDynamic.SetTextureParameterValue` _output_get_4 "Diffuse" _buttonrightgfx)
      (`MaterialInstanceDynamic.SetTextureParameterValue` _output_get_4 "Emissive Mask" _buttonrightgfx))))

(fn `SetRandomGroup`
  (set `self.ButtonGroup` (cast `/Game/Libraries/Minigames/E_EmailButtonGroup` (`KismetMathLibrary.Conv_IntToByte` (`KismetMathLibrary.RandomInteger` 4)))))

(fn `UserConstructionScript`)