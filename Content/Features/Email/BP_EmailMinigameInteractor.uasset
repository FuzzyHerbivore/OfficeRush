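; Interactor pawn for the email minigame, which an authorized player possesses to clear puzzle codes with directional inputs.
; On interaction it checks authorization, caches the player pawn, swaps input mapping contexts and snaps the character to the desk.
; FilterInput compares presses to the first code, removing matches until won or signalling mistakes with vibration.
; Canceling restores the cached pawn and resets the minigame; the glitch post-process setup is disconnected.
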(event `self.ReceiveBeginPlay`
  ; Post Process Setup
)

(event `HandleStampIncorrect`
  (params (FailedPlayer :type "/Game/Features/Stamping/ToPlace/BP_StampMinigameInteractor Object Reference"))
  ; Post Process Intensity
  (if (== FailedPlayer self)
    (bind (_direction _blend_weight) (`Timeline|Timeline` :!via `PlayFromStart`)
      (:`Update`
        (`MaterialInstanceDynamic.SetScalarParameterValue` (`self.Dynamic Glitch Material`) "Intensity" _blend_weight)))))

(event `EnhancedInput|/Game/UX/IA_Canceling`
  (params (ActionValue :type Boolean) (ElapsedSeconds :type "Float (double-precision)") (TriggeredSeconds :type "Float (double-precision)") (InputAction :type "InputAction Object Reference" :default "/Game/UX/IA_Canceling.IA_Canceling"))
  ; Exit Minigame
  (:`Triggered`
    (`self.ExitMinigame`)
    (`/Game/Features/Email/BP_EmailMinigame.SpawnPuzzleCodes` (`self.EmailMinigameRef`))))

(event `Event Possess Interactor`
  (params (Interactor :type "Actor Object Reference"))
  (bind _emailminigameref (`self.EmailMinigameRef`))
  (bind (_authorizedtokens_datatable _authorizedtokens_rowname) (break `DataTableRowHandle` (`/Game/Features/Email/BP_EmailMinigame.AuthorizedTokens` (`self.EmailMinigameRef`))))
  (bind _playercontrollerref (`/Game/Features/Email/BP_EmailMinigame.PlayerControllerRef` (`self.EmailMinigameRef`)))
  (bind _returnvalue (pcsubsystem `EnhancedInputLocalPlayerSubsystem` _playercontrollerref))
  ; Take control of this pawn if authorized
  (bind _asbpi_authorizer (cast `/Game/Libraries/Authorization/BPI_Authorizer` Interactor))
  (bind _returnvalue_2 (`|GetDataTableRow` "/Game/Libraries/Authorization/DT_AuthorizationTokens.DT_AuthorizationTokens" _authorizedtokens_rowname)
    (:`then`
      (bind _isauthorized (`/Game/Libraries/Authorization/BPI_Authorizer.CheckAuthorization` _asbpi_authorizer (`|MakeArray` _returnvalue_2)))
      (if _isauthorized
        (`|ExecutionSequence`
          (:`then_0`
            ; Cache the previous Pawn
            (bind _aspawn (cast `Pawn` Interactor))
            (bind _asbpi_cache (cast `/Game/Libraries/Cache/BPI_Cache` (`self.GetController` _aspawn)))
            (`/Game/Libraries/Cache/BPI_Cache.Cache` _asbpi_cache Interactor))
          (:`then_1`
            (bind _asbpi_controller (cast `/Game/Libraries/Controlling/BPI_Controller` Interactor))
            (`/Game/Libraries/Controlling/BPI_Controller.TakeControl` _asbpi_controller self)
            (`EnhancedInputSubsystemInterface.AddMappingContext` _returnvalue "/Game/Input/IMC_Tasks.IMC_Tasks" 0 (struct))
            (`EnhancedInputSubsystemInterface.RemoveMappingContext` _returnvalue "/Game/Input/IMC_Default.IMC_Default" (struct))
            (`self.SetPlayerPosition`)
            (set `/Game/Features/Email/BP_EmailDesk.Interacted` true (`/Game/Features/Email/BP_EmailMinigame.EmailDesk` (`self.EmailMinigameRef`)))
            (set `/Game/Features/Email/BP_EmailMinigame.IsTimerStarted` true (`self.EmailMinigameRef`))
            (`/Game/Players/BP_PlayerController.OnMinigameEnteredOnce` _playercontrollerref 2)
            (`/Game/Players/BP_PlayerCharacter.Event MinigameEntered` (`/Game/Features/Email/BP_EmailMinigame.PlayerCharacterRef` (`self.EmailMinigameRef`)))))
        (else
          (`GameplayStatics.PlaySoundAtLocation` "/Game/SoundAndMusic/SoundEffects/InteractionSounds/MS_InteractionFail.MS_InteractionFail" (`self.K2_GetActorLocation`) (struct) 1.0 1.0 0.0 null null null null)
          (`PlayerController.PlayDynamicForceFeedback` (`/Game/Features/Email/BP_EmailMinigame.PlayerControllerRef` _emailminigameref) (`/Game/Features/Email/BP_EmailMinigame.VibrationIntensity` _emailminigameref) (`/Game/Features/Email/BP_EmailMinigame.NoAuthorizationVibrationDuration` _emailminigameref) true true true true))))))

(event `EnhancedInput|/Game/Input/Actions/IA_Up`
  (params (ActionValue :type Boolean) (ElapsedSeconds :type "Float (double-precision)") (TriggeredSeconds :type "Float (double-precision)") (InputAction :type "InputAction Object Reference" :default "/Game/Input/Actions/IA_Up.IA_Up"))
  (bind _emailminigameref (`self.EmailMinigameRef`))
  (bind _output (`|GetArrayItem` (`/Game/Features/Email/BP_EmailMinigame.PuzzleCodes` (`self.EmailMinigameRef`))))
  (:`Started`
    (`/Engine/EditorBlueprintResources/StandardMacros.IsValid` _output
      (:`Is Valid`
        (bind _puzzlecodeoutput (`self.FilterInput` _output :!label _label)
          (:`Correct`
            (bind _out (`/Game/Features/Email/BP_EmailMinigame.CheckMinigameWon` (`self.EmailMinigameRef`)))
            (if (not _out)
              (`KismetSystemLibrary.PrintString` (`|GetEnumeratorNameAsString` (`/Game/Features/Email/BP_EmailButtonPreview.ButtonGroup` _puzzlecodeoutput)))
              (`/Game/Features/Email/BP_EmailMinigame.RemovePuzzleCode` (`self.EmailMinigameRef`) _puzzlecodeoutput)
              (bind _out_2 (`/Game/Features/Email/BP_EmailMinigame.CheckMinigameWon` (`self.EmailMinigameRef`)))
              (if _out_2
                (`/Game/Features/Email/BP_EmailMinigame.Event GameWon` (`self.EmailMinigameRef`))
                (else
                  (`/Game/Features/Email/BP_EmailMinigame.SetPuzzleCodePositions` (`self.EmailMinigameRef`))))))
          (:`Incorrect`
            (`/Game/Features/Email/BP_EmailMinigame.PressedWrongInput` _emailminigameref)
            (`PlayerController.PlayDynamicForceFeedback` (`/Game/Features/Email/BP_EmailMinigame.PlayerControllerRef` _emailminigameref) (`/Game/Features/Email/BP_EmailMinigame.VibrationIntensity` _emailminigameref) (`/Game/Features/Email/BP_EmailMinigame.IncorrectInputVibractionDuration` _emailminigameref) true true true true)))))))

(event `EnhancedInput|/Game/Input/Actions/IA_Down`
  (params (ActionValue :type Boolean) (ElapsedSeconds :type "Float (double-precision)") (TriggeredSeconds :type "Float (double-precision)") (InputAction :type "InputAction Object Reference" :default "/Game/Input/Actions/IA_Down.IA_Down"))
  (:`Started`
    (`/Engine/EditorBlueprintResources/StandardMacros.IsValid` (`|GetArrayItem` (`/Game/Features/Email/BP_EmailMinigame.PuzzleCodes` (`self.EmailMinigameRef`)))
      (:`Is Valid`
        (goto _label :!via `Down`)))))

(event `EnhancedInput|/Game/Input/Actions/IA_Left`
  (params (ActionValue :type Boolean) (ElapsedSeconds :type "Float (double-precision)") (TriggeredSeconds :type "Float (double-precision)") (InputAction :type "InputAction Object Reference" :default "/Game/Input/Actions/IA_Left.IA_Left"))
  (:`Started`
    (`/Engine/EditorBlueprintResources/StandardMacros.IsValid` (`|GetArrayItem` (`/Game/Features/Email/BP_EmailMinigame.PuzzleCodes` (`self.EmailMinigameRef`)))
      (:`Is Valid`
        (goto _label :!via `Left`)))))

(event `EnhancedInput|/Game/Input/Actions/IA_Right`
  (params (ActionValue :type Boolean) (ElapsedSeconds :type "Float (double-precision)") (TriggeredSeconds :type "Float (double-precision)") (InputAction :type "InputAction Object Reference" :default "/Game/Input/Actions/IA_Right.IA_Right"))
  (:`Started`
    (`/Engine/EditorBlueprintResources/StandardMacros.IsValid` (`|GetArrayItem` (`/Game/Features/Email/BP_EmailMinigame.PuzzleCodes` (`self.EmailMinigameRef`)))
      (:`Is Valid`
        (goto _label :!via `Right`)))))

(fn `ExitMinigame`
  (bind _returnvalue (`self.GetController`))
  (bind _playercontrollerref (`/Game/Features/Email/BP_EmailMinigame.PlayerControllerRef` (`self.EmailMinigameRef`)))
  (bind _returnvalue_2 (pcsubsystem `EnhancedInputLocalPlayerSubsystem` (`/Game/Features/Email/BP_EmailMinigame.PlayerControllerRef` (`self.EmailMinigameRef`))))
  (set `self.IsInteracting` false)
  (bind _asbpi_cache (cast `/Game/Libraries/Cache/BPI_Cache` _returnvalue))
  (bind _actor (`/Game/Libraries/Cache/BPI_Cache.Retrieve` _asbpi_cache))
  (bind _aspawn (cast `Pawn` _actor))
  (`Controller.Possess` _returnvalue _aspawn)
  (`EnhancedInputSubsystemInterface.AddMappingContext` _returnvalue_2 "/Game/Input/IMC_Default.IMC_Default" 0 (struct))
  (`EnhancedInputSubsystemInterface.RemoveMappingContext` _returnvalue_2 "/Game/Input/IMC_Tasks.IMC_Tasks" (struct))
  (set `/Game/Features/Email/BP_EmailDesk.Interacted` false (`/Game/Features/Email/BP_EmailMinigame.EmailDesk` (`self.EmailMinigameRef`)))
  (`/Game/Features/Email/BP_EmailMinigame.ResetMinigame` (`self.EmailMinigameRef`))
  (`/Game/Players/BP_PlayerController.OnTaskCompletedOnce` _playercontrollerref (`GameplayStatics.GetPlayerControllerID` _playercontrollerref))
  (`/Game/Players/BP_PlayerCharacter.Event MinigameExited` (`/Game/Features/Email/BP_EmailMinigame.PlayerCharacterRef` (`self.EmailMinigameRef`))))

(fn `SetPlayerPosition`
  (bind _emailminigameref (`self.EmailMinigameRef`))
  (bind _playerstandlocation (`/Game/Features/Email/BP_EmailMinigame.PlayerStandLocation` _emailminigameref))
  (`self.K2_SetActorLocationAndRotation` (`/Game/Features/Email/BP_EmailMinigame.PlayerCharacterRef` _emailminigameref) (`SceneComponent.K2_GetComponentLocation` _playerstandlocation) (`SceneComponent.K2_GetComponentRotation` _playerstandlocation) false true))

(fn `UserConstructionScript`)