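; NPC character that stalls stallable actors on collision, playing chatter, a montage and a speech bubble while turning to face them.
; ACStaller drives the stall, revealing a bubble button when ready so Interact can release it and restore rotation.
; Tick yaws the bubble toward the camera and polls DetectionRange, toggling a timeline-animated Niagara scan warning when stallables are nearby.
; Shoves pass to ACShovable unless the NPC is falling.
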(event `self.ReceiveTick`
  (params (DeltaSeconds :type "Float (single-precision)"))
  (`self.CheckForAlertVisibilityUpdate`)
  (`self.UpdateSpeechbubbleRotation`))

(event `self.ReceiveBeginPlay`
  (bind _chattersource (`self.ChatterSource`))
  ; Setup Visuals
  (`ActorComponent.Deactivate` (`self.CollisionRangeIndicatorFXS`))
  (if (`AudioComponent.IsPlaying` _chattersource)
    (`AudioComponent.Stop` _chattersource)))

(event `self.Shove`
  (params (ShovingActor :type "Actor Object Reference (by ref)"))
  ; Get Shoved
  (if (not (`NavMovementComponent.IsFalling` (`self.CharacterMovement`)))
    (`/Game/Features/Shoving/AC_Shovable.ReactToShove` (`self.AC_Shovable`) ShovingActor)))

(event `/Game/Libraries/Interaction/BPI_Interactable.Interact`
  (params (Interactor :type "Actor Object Reference (by ref)"))
  ; Interaction
  (bind _isstalling (`/Game/Features/NPCs/Stalling/AC_Staller.CheckIsStalling` (`self.AC_Staller`)))
  (if _isstalling
    (bind _aswbp_speech_bubble (cast `/Game/Vfx/StallingEffect/WBP_SpeechBubble` (`WidgetComponent.GetUserWidgetObject` (`self.Speechbubble`))))
    (bind _isshowingbutton (`/Game/Vfx/StallingEffect/WBP_SpeechBubble.CheckIsShowingButton` _aswbp_speech_bubble))
    (if _isshowingbutton
      (`/Game/Vfx/StallingEffect/WBP_SpeechBubble.HideButton` _aswbp_speech_bubble)
      (`/Game/Features/NPCs/Stalling/AC_Staller.DoUnstall` (`self.AC_Staller`)))))

(event `self.ReceiveHit`
  (params (MyComp :type "PrimitiveComponent Object Reference") (Other :type "Actor Object Reference") (OtherComp :type "PrimitiveComponent Object Reference") (bSelfMoved :type Boolean) (HitLocation :type "Vector Structure") (HitNormal :type "Vector Structure") (NormalImpulse :type "Vector Structure") (Hit :type "HitResult Structure (by ref)"))
  ; Stall actor on being hit
  (bind _isstalling (`/Game/Features/NPCs/Stalling/AC_Staller.CheckIsStalling` (`self.AC_Staller`)))
  (if (not _isstalling)
    (bind _asbpi_stallable (cast `/Game/Features/NPCs/Stalling/BPI_Stallable` Other))
    (bind _didstallsuccessfully (`/Game/Features/NPCs/Stalling/AC_Staller.DoStall` (`self.AC_Staller`) _asbpi_stallable))
    (if _didstallsuccessfully
      (add `/Game/Features/NPCs/Stalling/AC_Staller.ReadyToUnstall` (`self.AC_Staller`) (delegate `StartConfirmToUnstall`)))))

(event `StartConfirmToUnstall`
  ; Stall actor on being hit
  (bind _aswbp_speech_bubble (cast `/Game/Vfx/StallingEffect/WBP_SpeechBubble` (`WidgetComponent.GetUserWidgetObject` (`self.Speechbubble`))))
  (`/Game/Vfx/StallingEffect/WBP_SpeechBubble.ShowButton` _aswbp_speech_bubble))

(event `self.AC_Staller.DidStall`
  (params (Stallable :type "/Game/Features/NPCs/Stalling/BPI_Stallable Interface"))
  ; Stall actor on being hit
  (`self.PlayAnimMontage` "/Game/Characters/Animations/ME_Char_NPC_Stall_V02_Montage.ME_Char_NPC_Stall_V02_Montage")
  (`AudioComponent.Play` (`self.ChatterSource`) 0.0)
  (`SceneComponent.SetVisibility` (`self.Speechbubble`) true true)
  (bind _location (`/Game/Features/NPCs/Stalling/BPI_Stallable.GetStallableLocation` Stallable))
  (bind _output_get (set `self.InitialRotation` (`self.K2_GetActorRotation`)))
  (bind (_direction _rotationlerpalpha) (`Timeline|StallRotationTimeline` :!via `PlayFromStart`)
    (:`Update`
      (`self.K2_SetActorRotation` (`KismetMathLibrary.RLerp` _output_get (`KismetMathLibrary.FindLookAtRotation` (`self.K2_GetActorLocation`) _location) _rotationlerpalpha)))))

(event `self.AC_Staller.DidUnstall`
  ; Stall actor on being hit
  (`SceneComponent.SetVisibility` (`self.Speechbubble`) false true)
  (bind (_direction _rotationlerpalpha) (`Timeline|UnstallRotationTimeline` :!via `PlayFromStart`)
    (:`Update`
      (`self.K2_SetActorRotation` (`KismetMathLibrary.RLerp` (`self.K2_GetActorRotation`) (`self.InitialRotation`) _rotationlerpalpha)))))

(event `UpdateSpeechbubbleRotation`
  (bind _speechbubble (`self.Speechbubble`))
  (bind (_returnvalue_roll _returnvalue_pitch _returnvalue_yaw) (`KismetMathLibrary.BreakRotator` (`KismetMathLibrary.FindLookAtRotation` (`SceneComponent.K2_GetComponentLocation` _speechbubble) (`SceneComponent.K2_GetComponentLocation` (`PlayerCameraManager.TransformComponent` (`GameplayStatics.GetPlayerCameraManager` 0))))))
  ; Stall actor on being hit
  (`SceneComponent.K2_SetWorldRotation` _speechbubble (`KismetMathLibrary.MakeRotator` 0.0 0.0 _returnvalue_yaw) false false))

(event `CheckForAlertVisibilityUpdate`
  ; Stall telegraphing
  (bind _arestallablesinrange (`self.CheckForStallables`))
  (if (not (== _arestallablesinrange (`self.AreStallablesInRange`)))
    (bind _output_get (set `self.AreStallablesInRange` _arestallablesinrange))
    (`self.UpdateAlertVisibility` _output_get)))

(event `UpdateAlertVisibility`
  (params (IsVisible :type Boolean))
  ; Stall telegraphing
  (if IsVisible
    (`|ExecutionSequence`
      (:`then_0`
        (`FXSystemComponent.SetFloatParameter` (`self.CollisionRangeIndicatorFXS`) "User.EmissiveStrengthScan" 0.0))
      (:`then_1`
        (`ActorComponent.Activate` (`self.CollisionRangeIndicatorFXS`) false)
        (`FXSystemComponent.SetVectorParameter` (`self.CollisionRangeIndicatorFXS`) "User.Position03" (0.0 0.0 180.0))
        (bind (_direction _newtrack_0) (`Timeline|StartScan` :!via `PlayFromStart`)
          (:`Update`
            (`FXSystemComponent.SetVectorParameter` (`self.CollisionRangeIndicatorFXS`) "User.ShapeLSize" (`KismetMathLibrary.MakeVector` _newtrack_0 _newtrack_0 _newtrack_0)))
          (:`Finished`
            (`FXSystemComponent.SetFloatParameter` (`self.CollisionRangeIndicatorFXS`) "User.EmissiveStrengthScan" 10.0)
            (bind (_direction_2 _heighttop) (`Timeline|ScanContinuous` :!via `PlayFromStart`)
              (:`Update`
                (`FXSystemComponent.SetVectorParameter` (`self.CollisionRangeIndicatorFXS`) "User.Position03" (`KismetMathLibrary.MakeVector` 0.0 0.0 _heighttop))))))))
    (else
      (bind (_direction_3 _newtrack_0_2) (`Timeline|Timeline` :!via `ReverseFromEnd`)
        (:`Update`
          (`FXSystemComponent.SetVectorParameter` (`self.CollisionRangeIndicatorFXS`) "User.ShapeLSize" (`KismetMathLibrary.MakeVector` _newtrack_0_2 _newtrack_0_2 _newtrack_0_2)))
        (:`Finished`
          (`ActorComponent.Deactivate` (`self.CollisionRangeIndicatorFXS`)))))))

(fn `CheckForStallables`
  (returns (AreStallablesInRange :type Boolean))
  (locals (Stallables :type "Array of /Game/Features/NPCs/Stalling/BPI_Stallable Interface"))
  (for _array_element (`PrimitiveComponent.GetOverlappingActors` (`self.DetectionRange`) null)
    (bind _asbpi_stallable (cast `/Game/Features/NPCs/Stalling/BPI_Stallable` _array_element))
    (bind _isstallable (`/Game/Features/NPCs/Stalling/BPI_Stallable.CheckIsStallable` _asbpi_stallable))
    (if _isstallable
      (`KismetArrayLibrary.Array_AddUnique` (`local.Stallables`) _asbpi_stallable)))
  (return (`KismetArrayLibrary.Array_IsNotEmpty` (`local.Stallables`))))

(fn `GetActor`
  (returns (Actor :type "Actor Object Reference"))
  (return self))

(fn `UserConstructionScript`)