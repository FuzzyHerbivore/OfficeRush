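; Actor component that lets its owner, likely an NPC, be stalled by another party, with a cooldown between stalls.
; BeStalled succeeds only when the owner is neither stalled nor cooling down, then records the state, fires StallStarted with the instigator and reports the result.
; BeUnstalled clears the state, fires StallFinished and starts a timer whose handle validity serves as the cooldown flag until expiry invalidates it and fires StallCooldownFinished.
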(event `BeUnstalled`
  ; AC_Stallable
  (set `self.IsStalled` false)
  (bind _returnvalue (`KismetSystemLibrary.K2_SetTimerDelegate` (delegate `InvalidateCooldownTimer`) (`self.StallCooldownDuration`)))
  (set `self.StallCooldownTimerHandle` _returnvalue)
  (`self.StallFinished`))

(event `InvalidateCooldownTimer`
  ; AC_Stallable
  (`KismetSystemLibrary.K2_ClearAndInvalidateTimerHandle` (`self.StallCooldownTimerHandle`))
  (`self.StallCooldownFinished`))

(fn `BeStalled`
  (params (StalledBy :type "/Game/Features/NPCs/Stalling/AC_Staller Object Reference"))
  (returns (WasStalledSuccessfully :type Boolean))
  (bind _isstallable (`self.CheckIsStallable`))
  (if _isstallable
    (set `self.IsStalled` true)
    (`self.StallStarted` StalledBy)
    (return true)
    (else
      (return false))))

(fn `CheckIsInStallCooldown`
  (returns (IsInCooldown :type Boolean))
  (return (`KismetSystemLibrary.K2_IsValidTimerHandle` (`self.StallCooldownTimerHandle`))))

(fn `CheckIsStallable`
  (returns (IsStallable :type Boolean))
  (bind _isstalled (`self.CheckIsStalled`))
  (bind _isincooldown (`self.CheckIsInStallCooldown`))
  (return (and (not _isincooldown) (not _isstalled))))

(fn `CheckIsStalled`
  (returns (IsStalled :type Boolean))
  (return (`self.IsStalled`)))