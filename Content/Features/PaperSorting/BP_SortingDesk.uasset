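; BP_SortingDesk is an interactable desk that hands the player into the paper sorting minigame.
; On Interact, if not already in use, it passes the player character and its controller to the referenced minigame, then calls EventPossesMinigame on it.
; IsInteracted sets the in-use flag and mirrors it onto the player's InteractedWithMinigame, while GetActor returns the desk itself.
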(event `self.ReceiveBeginPlay`)

(event `/Game/Libraries/Interaction/BPI_Interactable.Interact`
  (params (Interactor :type "Actor Object Reference (by ref)"))
  (bind _sortingminigameref (`self.SortingMinigameRef`))
  (if (not (`self.Interacted`))
    (bind _asbp_player_character (cast `/Game/Players/BP_PlayerCharacter` Interactor))
    (bind _output_get (set `self.PlayerReference` _asbp_player_character))
    (bind _output_get_2 (set `/Game/Features/PaperSorting/BP_SortingMinigame.PlayerCharacterRef` _output_get (`self.SortingMinigameRef`)))
    (bind _asbp_player_controller (cast `/Game/Players/BP_PlayerController` (`self.GetController` _output_get_2)))
    (set `/Game/Features/PaperSorting/BP_SortingMinigame.PlayerControllerRef` _asbp_player_controller _sortingminigameref)
    (`/Game/Features/PaperSorting/BP_SortingMinigame.Event PossesMinigame` _sortingminigameref Interactor)))

(fn `GetActor`
  (returns (Actor :type "Actor Object Reference"))
  (return self))

(fn `IsInteracted`
  (params (value :type Boolean) (player :type "/Game/Players/BP_PlayerCharacter Object Reference"))
  (bind _output_get (set `self.Interacted` value))
  (set `/Game/Players/BP_PlayerCharacter.InteractedWithMinigame` _output_get player))

(fn `UserConstructionScript`)