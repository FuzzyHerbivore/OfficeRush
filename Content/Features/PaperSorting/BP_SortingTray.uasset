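; BP_SortingTray is a color-coded tray in the paper sorting minigame that accepts papers matching its sorting group.
; On BeginPlay it creates a dynamic material instance and tints it for its Blue, Red or Green group.
; Overlapping matching papers notify the minigame, snap onto a stack point that rises with each paper, and stop simulating physics; mismatches play a fail sound.
; A Hovered event toggles the tray's glow strength.
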(event `self.ReceiveBeginPlay`
  (bind _me_envi_papertray (`self.ME_Envi_PaperTray`))
  (bind _returnvalue (`PrimitiveComponent.CreateDynamicMaterialInstance` _me_envi_papertray 0 (`PrimitiveComponent.GetMaterial` _me_envi_papertray 0) "None"))
  (set `self.StampDynamicMaterialInstance` _returnvalue)
  (`self.SetTrayColor`))

(event `self.PaperTrigger.OnComponentBeginOverlap`
  (params (OverlappedComponent :type "PrimitiveComponent Object Reference") (OtherActor :type "Actor Object Reference") (OtherComp :type "PrimitiveComponent Object Reference") (OtherBodyIndex :type Integer) (bFromSweep :type Boolean) (SweepResult :type "HitResult Structure (by ref)"))
  (if (== (`GameplayStatics.GetObjectClass` OtherActor) "/Game/Features/PaperSorting/BP_SortingPaper.BP_SortingPaper_C")
    (bind _asbp_sorting_paper (cast `/Game/Features/PaperSorting/BP_SortingPaper` OtherActor))
    (if (`|EnumEquality` (`/Game/Features/PaperSorting/BP_SortingPaper.PaperSortingGroup` _asbp_sorting_paper) (`self.PaperSortingGroup`))
      (`GameplayStatics.PlaySoundAtLocation` "/Game/SoundAndMusic/SoundEffects/MiniGames/MS_ActionSuccess.MS_ActionSuccess" (`self.K2_GetActorLocation`) (struct) 1.0 1.0 0.0 null null null null)
      (`/Game/Features/PaperSorting/BP_SortingMinigame.Event CorrectPaper` (`self.MinigameRef`) _asbp_sorting_paper)
      (`self.K2_SetActorLocationAndRotation` _asbp_sorting_paper (`SceneComponent.K2_GetComponentLocation` (`self.PaperMoveLocation`)) (`/Game/Features/PaperSorting/BP_SortingPaper.OriginalRotation` _asbp_sorting_paper) false false)
      (`PrimitiveComponent.SetSimulatePhysics` (`/Game/Features/PaperSorting/BP_SortingPaper.Paper` _asbp_sorting_paper) false)
      (`SceneComponent.K2_AddWorldOffset` (`self.PaperMoveLocation`) (`KismetMathLibrary.MakeVector` 0.0 0.0 (* (.z (`.BoxExtent` (`self.GetActorBounds` _asbp_sorting_paper false false))) 4.0)) false false)
      (else
        (`GameplayStatics.PlaySoundAtLocation` "/Game/SoundAndMusic/SoundEffects/MiniGames/MS_ActionFail.MS_ActionFail" (`self.K2_GetActorLocation`) (struct) 1.0 1.0 0.0 null null null null)))))

(event `/Game/Features/Stamping/BPI_Hoverable.Hovered`
  (params (Hovered :type Boolean))
  (if Hovered
    (`MaterialInstanceDynamic.SetScalarParameterValue` (`self.StampDynamicMaterialInstance`) "GlowStrainght" 5.0)
    (else
      (`MaterialInstanceDynamic.SetScalarParameterValue` (`self.StampDynamicMaterialInstance`) "GlowStrainght" 0.5))))

(fn `SetTrayColor`
  (returns (SortingGroup :type "/Game/Features/PaperSorting/E_PaperSortingGroups Enum"))
  (bind _papersortinggroup (`self.PaperSortingGroup`))
  (bind _stampdynamicmaterialinstance (`self.StampDynamicMaterialInstance`))
  (bind _stampdynamicmaterialinstance_2 (`self.StampDynamicMaterialInstance`))
  (bind _stampdynamicmaterialinstance_3 (`self.StampDynamicMaterialInstance`))
  (`|ExecutionSequence`
    (:`then_0`
      (switch `/Game/Features/PaperSorting/E_PaperSortingGroups` _papersortinggroup
        (:`NewEnumerator0`
          (bind _output_get (set `self.PaperColor` 1.5))
          (`MaterialInstanceDynamic.SetScalarParameterValue` _stampdynamicmaterialinstance "TintColor LUT" _output_get)
          (`MaterialInstanceDynamic.SetScalarParameterValue` _stampdynamicmaterialinstance "EmissiveColor LUT" 1.0))
        (:`NewEnumerator1`
          (bind _output_get_2 (set `self.PaperColor` 5.1))
          (`MaterialInstanceDynamic.SetScalarParameterValue` _stampdynamicmaterialinstance_2 "TintColor LUT" _output_get_2)
          (`MaterialInstanceDynamic.SetScalarParameterValue` _stampdynamicmaterialinstance_2 "EmissiveColor LUT" 1.0))
        (:`NewEnumerator2`
          (bind _output_get_3 (set `self.PaperColor` 3.1))
          (`MaterialInstanceDynamic.SetScalarParameterValue` _stampdynamicmaterialinstance_3 "TintColor LUT" _output_get_3)
          (`MaterialInstanceDynamic.SetScalarParameterValue` _stampdynamicmaterialinstance_3 "EmissiveColor LUT" 1.0))))
    (:`then_1`
      (return _papersortinggroup))))

(fn `UserConstructionScript`)