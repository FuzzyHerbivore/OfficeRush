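; Actor component that lets its owning Character be shoved, with a brief visual flash.
; ReactToShove launches the character upward and planar-away from the shoving actor using separate planar and vertical forces, then briefly raises overlay opacity.
; On BeginPlay it gives each skeletal mesh a hidden additive overlay material instance, but stores only the last one, so only that mesh flashes.
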(event `self.ReceiveBeginPlay`
  (`self.AddBeingShovedMaterial`))

(event `ReactToShove`
  (params (ShovingActor :type "Actor Object Reference"))
  (bind _returnvalue (`self.GetOwner`))
  (bind _shoveplanarforce (`self.ShovePlanarForce`))
  ; React To Shove
  (bind _ascharacter (cast `Character` _returnvalue))
  (`Character.LaunchCharacter` _ascharacter (* (`KismetMathLibrary.MakeVector` (.x (`KismetMathLibrary.Vector_Normal2D` (- (`Actor.K2_GetActorLocation` _returnvalue) (`Actor.K2_GetActorLocation` ShovingActor)))) (.y (`KismetMathLibrary.Vector_Normal2D` (- (`Actor.K2_GetActorLocation` _returnvalue) (`Actor.K2_GetActorLocation` ShovingActor)))) 1.0) (`KismetMathLibrary.MakeVector` _shoveplanarforce _shoveplanarforce (`self.ShoveVerticalForce`))) false false)
  (`MaterialInstanceDynamic.SetScalarParameterValue` (`self.OverlayMaterial`) "Opacity" 0.2)
  (`KismetSystemLibrary.Delay` 0.7)
  (`MaterialInstanceDynamic.SetScalarParameterValue` (`self.OverlayMaterial`) "Opacity" 0.0))

(fn `AddBeingShovedMaterial`
  (for _array_element (`Actor.K2_GetComponentsByClass` (`self.GetOwner`) "/Script/Engine.SkeletalMeshComponent")
    (`/Engine/EditorBlueprintResources/StandardMacros.IsValid` _array_element
      (:`Is Valid`
        (bind _returnvalue (`KismetMaterialLibrary.CreateDynamicMaterialInstance` "/Game/Vfx/Materials/ParentMaterials/M_VFX_Additive_Meshes.M_VFX_Additive_Meshes"))
        (bind _output_get (set `self.OverlayMaterial` _returnvalue))
        (`MaterialInstanceDynamic.SetScalarParameterValue` _output_get "Opacity" 0.0)
        (`MeshComponent.SetOverlayMaterial` _array_element _output_get)))))