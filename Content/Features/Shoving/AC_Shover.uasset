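; AC_Shover is a scene component that lets its owner shove the nearest shovable actor in front of it.
; A sphere trace along the component's forward vector finds the target, then a half-second delay precedes calling GetShoved through BPI_Shovable.
; A successful shove spawns a pooled Niagara impact effect aligned to the hit normal, plus force feedback when the owner is a player character.
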(event `ShoveNearestShovableInFront`
  (bind _returnvalue (`self.K2_GetComponentLocation`))
  ; Shove Nearest Shovable in Front
  (bind (_outhit _returnvalue_2) (`KismetSystemLibrary.SphereTraceSingle` :`Start` _returnvalue :`End` (+ _returnvalue (* (`KismetMathLibrary.GetForwardVector` (`self.K2_GetComponentRotation`)) (`self.TraceLength`))) :`Radius` (`self.TraceRadius`) :`TraceChannel` "TraceTypeQuery4" :`DrawTime` 0.2))
  (if _returnvalue_2
    (bind (_bblockinghit _binitialoverlap _time _distance _location _impactpoint _normal _impactnormal _physmat _hitactor) (`GameplayStatics.BreakHitResult` _outhit))
    (`/Engine/EditorBlueprintResources/StandardMacros.IsValid` _hitactor
      (:`Is Valid`
        (`KismetSystemLibrary.Delay` 0.5)
        (bind _asbpi_shovable (cast `/Game/Features/Shoving/BPI_Shovable` _hitactor))
        (`/Game/Features/Shoving/BPI_Shovable.GetShoved` _asbpi_shovable (`self.GetOwner`))
        (`self.SpawnShoveImpactVFX` _location _impactnormal)
        (bind _asbp_player_character (cast `/Game/Players/BP_PlayerCharacter` (`self.GetOwner`)))
        (bind _asbp_player_controller (cast `/Game/Players/BP_PlayerController` (`Pawn.GetController` _asbp_player_character)))
        (`PlayerController.PlayDynamicForceFeedback` _asbp_player_controller 1.0 0.35 true true true true)))))

(event `SpawnShoveImpactVFX`
  (params (HitLocation :type "Vector Structure") (HitNormal :type "Vector Structure"))
  ; Spawn Impact VFX
  (`NiagaraFunctionLibrary.SpawnSystemAtLocation` "/Game/Vfx/ParticleSystems/FXS_VFX_Impact_Push_01.FXS_VFX_Impact_Push_01" HitLocation (`KismetMathLibrary.Conv_VectorToRotator` HitNormal) (1.0 1.0 1.0) true true "AutoRelease"))