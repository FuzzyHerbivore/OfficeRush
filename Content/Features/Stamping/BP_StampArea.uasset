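; BP_StampArea is a stamp area for the Stamping feature, assigned to a Blue, Red or Green stamp group.
; RandomStampGroup picks one of the groups at random, and SetStampColor applies the matching VFX material to the StampArea component.
; Neither function is called within this Blueprint, and the construction script is empty.
; The DisableStampArea event destroys the StampArea component rather than the whole Blueprint instance.
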(event `Event DisableStampArea`
  (`ActorComponent.K2_DestroyComponent` (`self.StampArea`)))

(fn `RandomStampGroup`
  (set `self.StampGroup` (cast `/Game/Libraries/Minigames/E_StampGroup` (`KismetMathLibrary.Conv_IntToByte` (`KismetMathLibrary.RandomInteger` 3)))))

(fn `SetStampColor`
  (bind _stamparea (`self.StampArea`))
  (switch `/Game/Libraries/Minigames/E_StampGroup` (`self.StampGroup`)
    (:`NewEnumerator0`
      (`PrimitiveComponent.SetMaterial` _stamparea 0 "/Game/Vfx/Stamping/M_VFX_StampArea_Blue.M_VFX_StampArea_Blue"))
    (:`NewEnumerator1`
      (`PrimitiveComponent.SetMaterial` _stamparea 0 "/Game/Vfx/Stamping/M_VFX_StampArea_Red.M_VFX_StampArea_Red"))
    (:`NewEnumerator2`
      (`PrimitiveComponent.SetMaterial` _stamparea 0 "/Game/Vfx/Stamping/M_VFX_StampArea_Green.M_VFX_StampArea_Green"))))

(fn `UserConstructionScript`)