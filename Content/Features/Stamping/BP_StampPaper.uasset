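; Paper prop for the stamping minigame that the player drags with the cursor once MarkForFinished is set and until IsFinished.
; On BeginPlay it picks a random spawn layout, applies the matching paper texture through a dynamic material, and spawns one or two randomized BP_StampArea actors attached to the paper.
; Dragging suspends physics, resets rotation and clamps pickup height.
; Hovering plays a glow timeline and updates the minigame cursor.
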(event `self.ReceiveBeginPlay`
  (set `self.OriginalRotation` (`SceneComponent.K2_GetComponentRotation` (`self.Paper`)))
  (set `self.OriginalLocation` (`SceneComponent.K2_GetComponentLocation` (`self.Paper`)))
  (`self.SpawnPaperAreas`))

(event `/Game/Libraries/Minigames/BPI_MinigameInteractable.MinigameInteractedStart`
  (params (PlayerActor :type "Actor Object Reference") (CursorWorldLocation :type "Vector Structure") (CursorWorldDirection :type "Vector Structure") (CursorHitLocation :type "Vector Structure"))
  (bind _paper (`self.Paper`))
  (if (`self.MarkForFinished`)
    (if (not (`self.IsFinished`))
      (`PrimitiveComponent.SetSimulatePhysics` _paper false)
      (`SceneComponent.K2_SetWorldRotation` _paper (`self.OriginalRotation`) false false)
      (set `self.IsInteracting` true)
      (`/Game/Features/Stamping/ToPlace/BP_StampMinigame.Event CursorInteracts` (`self.StampMinigameRef`)))))

(event `/Game/Libraries/Minigames/BPI_MinigameInteractable.MinigameInteractedEnded`
  (params (PlayerActor :type "Actor Object Reference") (CursorWorldLocation :type "Vector Structure") (CursorWorldDirection :type "Vector Structure") (CursorHitLocation :type "Vector Structure"))
  (if (`self.MarkForFinished`)
    (if (not (`self.IsFinished`))
      (`PrimitiveComponent.SetSimulatePhysics` (`self.Paper`) true)
      (set `self.IsInteracting` false)
      (`/Game/Features/Stamping/ToPlace/BP_StampMinigame.Event CursorDefault` (`self.StampMinigameRef`)))))

(event `/Game/Libraries/Minigames/BPI_MinigameInteractable.MinigameInteractedContinous`
  (params (PlayerActor :type "Actor Object Reference") (CursorWorldLocation :type "Vector Structure") (CursorWorldDirection :type "Vector Structure") (CursorHitLocation :type "Vector Structure"))
  (bind (_returnvalue_x _returnvalue_y _returnvalue_z) (`KismetMathLibrary.BreakVector` (+ CursorWorldLocation CursorWorldDirection CursorHitLocation)))
  (bind (_itempickupheight_x _itempickupheight_y) (`KismetMathLibrary.BreakVector2D` (`/Game/Features/Stamping/ToPlace/BP_StampMinigame.ItemPickupHeight` (`self.StampMinigameRef`))))
  (if (`self.MarkForFinished`)
    (if (`self.IsFinished`)
      _
      (elif (`self.IsInteracting`)
        (`SceneComponent.K2_SetWorldLocation` (`self.Paper`) (`KismetMathLibrary.MakeVector` _returnvalue_x _returnvalue_y (`KismetMathLibrary.FClamp` _returnvalue_z _itempickupheight_x _itempickupheight_y)) false false)))))

(event `/Game/Features/Stamping/BPI_Hoverable.Hovered`
  (params (Hovered :type Boolean))
  (if (`self.MarkForFinished`)
    (if Hovered
      (`/Game/Features/Stamping/ToPlace/BP_StampMinigame.Event CursorHovers` (`self.StampMinigameRef`))
      (bind (_direction _newtrack_0) (`Timeline|Glow` :!label _label)
        (:`Update`
          (`MaterialInstanceDynamic.SetScalarParameterValue` (`self.PaperDMI`) "GlowStrainght" _newtrack_0)))
      (else
        (`/Game/Features/Stamping/ToPlace/BP_StampMinigame.Event CursorDefault` (`self.StampMinigameRef`))
        (goto _label :!via `Reverse`)))))

(fn `IsHovered`
  (params (in :type Boolean))
  (returns (out :type Boolean))
  (bind _output_get (set `self.bIsHovered` in))
  (return _output_get))

(fn `SelectPaperTexture`
  (params (Index :type Integer))
  (switch `int` Index
    (:`0`
      (bind _returnvalue (`PrimitiveComponent.CreateDynamicMaterialInstance` (`self.Paper`) 0 "/Game/Features/Stamping/M_Inst_StampPaper.M_Inst_StampPaper" "None"))
      (bind _output_get (set `self.PaperDMI` _returnvalue))
      (`MaterialInstanceDynamic.SetTextureParameterValue` _output_get "Diffuse" "/Game/Environment/Assets/Paper/1/T_Envi_Paper1_BaseColor_V03.T_Envi_Paper1_BaseColor_V03")
      (`MaterialInstanceDynamic.SetTextureParameterValue` _output_get "Emissive Mask" "/Game/Environment/Assets/Paper/1/T_Envi_Paper1_Emissive_V03.T_Envi_Paper1_Emissive_V03"))
    (:`1`
      (bind _returnvalue_2 (`PrimitiveComponent.CreateDynamicMaterialInstance` (`self.Paper`) 0 "/Game/Features/Stamping/M_Inst_StampPaper.M_Inst_StampPaper" "None"))
      (bind _output_get_2 (set `self.PaperDMI` _returnvalue_2))
      (`MaterialInstanceDynamic.SetTextureParameterValue` _output_get_2 "Diffuse" "/Game/Environment/Assets/Paper/2/T_Envi_Paper2_BaseColor_V03.T_Envi_Paper2_BaseColor_V03")
      (`MaterialInstanceDynamic.SetTextureParameterValue` _output_get_2 "Emissive Mask" "/Game/Environment/Assets/Paper/2/T_Envi_Paper2_Emissive_V03.T_Envi_Paper2_Emissive_V03"))
    (:`2`
      (bind _returnvalue_3 (`PrimitiveComponent.CreateDynamicMaterialInstance` (`self.Paper`) 0 "/Game/Features/Stamping/M_Inst_StampPaper.M_Inst_StampPaper" "None"))
      (bind _output_get_3 (set `self.PaperDMI` _returnvalue_3))
      (`MaterialInstanceDynamic.SetTextureParameterValue` _output_get_3 "Diffuse" "/Game/Environment/Assets/Paper/3/T_Envi_Paper3_BaseColor_V03.T_Envi_Paper3_BaseColor_V03")
      (`MaterialInstanceDynamic.SetTextureParameterValue` _output_get_3 "Emissive Mask" "/Game/Environment/Assets/Paper/3/T_Envi_Paper3_Emissive_V03.T_Envi_Paper3_Emissive_V03"))
    (:`3`
      (bind _returnvalue_4 (`PrimitiveComponent.CreateDynamicMaterialInstance` (`self.Paper`) 0 "/Game/Features/Stamping/M_Inst_StampPaper.M_Inst_StampPaper" "None"))
      (bind _output_get_4 (set `self.PaperDMI` _returnvalue_4))
      (`MaterialInstanceDynamic.SetTextureParameterValue` _output_get_4 "Diffuse" "/Game/Environment/Assets/Paper/4/T_Envi_Paper4_BaseColor_V03.T_Envi_Paper4_BaseColor_V03")
      (`MaterialInstanceDynamic.SetTextureParameterValue` _output_get_4 "Emissive Mask" "/Game/Environment/Assets/Paper/4/T_Envi_Paper4_Emissive_V03.T_Envi_Paper4_Emissive_V03"))
    (:`4`
      (bind _returnvalue_5 (`PrimitiveComponent.CreateDynamicMaterialInstance` (`self.Paper`) 0 "/Game/Features/Stamping/M_Inst_StampPaper.M_Inst_StampPaper" "None"))
      (bind _output_get_5 (set `self.PaperDMI` _returnvalue_5))
      (`MaterialInstanceDynamic.SetTextureParameterValue` _output_get_5 "Diffuse" "/Game/Environment/Assets/Paper/5/T_Envi_Paper5_BaseColor_V03.T_Envi_Paper5_BaseColor_V03")
      (`MaterialInstanceDynamic.SetTextureParameterValue` _output_get_5 "Emissive Mask" "/Game/Environment/Assets/Paper/5/T_Envi_Paper5_Emissive_V03.T_Envi_Paper5_Emissive_V03")))
  (`MaterialInstanceDynamic.SetScalarParameterValue` (`self.PaperDMI`) "GlowStrainght" 0.4))

(fn `Spawn`
  (params (input :type "SceneComponent Object Reference"))
  (bind (_returnvalue_location _returnvalue_rotation) (`KismetMathLibrary.BreakTransform` (`SceneComponent.K2_GetComponentToWorld` input)))
  (bind _returnvalue (`|SpawnActorFromClass` "/Game/Features/Stamping/BP_StampArea.BP_StampArea_C" (`KismetMathLibrary.MakeTransform` _returnvalue_location _returnvalue_rotation) "Undefined" "MultiplyWithRoot" null null))
  (`/Game/Features/Stamping/BP_StampArea.RandomStampGroup` _returnvalue)
  (`/Game/Features/Stamping/BP_StampArea.SetStampColor` _returnvalue)
  (`KismetArrayLibrary.Array_Add` (`self.SpawnedStampArray`) _returnvalue)
  (`self.K2_AttachToComponent` _returnvalue (`self.Paper`) "None" "KeepWorld" "KeepWorld" "KeepWorld" true)
  (bind (_returnvalue_x _returnvalue_y _returnvalue_z) (`KismetMathLibrary.BreakVector` (`self.K2_GetActorLocation` _returnvalue)))
  (`self.K2_SetActorLocation` _returnvalue (`KismetMathLibrary.MakeVector` _returnvalue_x _returnvalue_y (+ _returnvalue_z 0.2)) false false))

(fn `SpawnPaperAreas`
  (bind _spawnindex (`self.SpawnIndex`))
  (bind _array (`|MakeArray` (`self.BP_StampAreaSpawnLocation1`) (`self.BP_StampAreaSpawnLocation2`) (`self.BP_StampAreaSpawnLocation3`) (`self.BP_StampAreaSpawnLocation4`) (`self.BP_StampAreaSpawnLocation5`)))
  (bind _result (`/Engine/EditorBlueprintResources/StandardMacros.DecrementInt` (`KismetArrayLibrary.Array_Length` _array))
    (:`  `
      (set `self.SpawnIndex` (`KismetMathLibrary.RandomIntegerInRange` 0 _result))
      (`self.SelectPaperTexture` _spawnindex)
      (set `self.StampAreaArray` (`|MakeArray` (`|GetArrayItem` _array _spawnindex) (`KismetArrayLibrary.Array_Random` (`|MakeArray` (`self.BP_StampAreaSpawnLocation6`) (`self.BP_StampAreaSpawnLocation7`) (`self.BP_StampAreaSpawnLocation8`))) :!type "SceneComponent Object Reference"))
      (if (`KismetMathLibrary.RandomBool`)
        (bind _output_get (set `self.StampAmount` 1))
        (bind _result_2 (`/Engine/EditorBlueprintResources/StandardMacros.DecrementInt` _output_get)
          (:`  `
            (`self.Spawn` (`|GetArrayItem` (`self.StampAreaArray`) _result_2))
            (`/Engine/EditorBlueprintResources/StandardMacros.IncrementInt` (`self.StampAmount`))))
        (else
          (bind _output_get_2 (set `self.StampAmount` 2))
          (bind _result_3 (`/Engine/EditorBlueprintResources/StandardMacros.DecrementInt` _output_get_2)
            (:`  `
              (for _index (range (+ _result_3 1))
                (`self.Spawn` (`|GetArrayItem` (`self.StampAreaArray`) _index)))
              (`/Engine/EditorBlueprintResources/StandardMacros.IncrementInt` (`self.StampAmount`)))))))))

(fn `UserConstructionScript`)