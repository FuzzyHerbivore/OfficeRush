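; Interactable stamp desk that hands the player over to the stamping minigame.
; On Interact, while not already in use, it passes the player character and controller to the referenced minigame and calls its possess event.
; IsInteracted sets the desk's in-use flag and mirrors it to the player's InteractedWithMinigame, while GetActor returns the desk itself.
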(event `self.ReceiveBeginPlay`)

(event `/Game/Libraries/Interaction/BPI_Interactable.Interact`
  (params (Interactor :type "Actor Object Reference (by ref)"))
  (bind _stampminigameref (`self.StampMinigameRef`))
  (bind _playerreference (`self.PlayerReference`))
  (if (not (`self.Interacted`))
    (bind _asbp_player_character (cast `/Game/Players/BP_PlayerCharacter` Interactor))
    (set `self.PlayerReference` _asbp_player_character)
    (set `/Game/Features/Stamping/ToPlace/BP_StampMinigame.PlayerCharacterRef` _playerreference (`self.StampMinigameRef`))
    (bind _asbp_player_controller (cast `/Game/Players/BP_PlayerController` (`self.GetController` _playerreference)))
    (set `/Game/Features/Stamping/ToPlace/BP_StampMinigame.PlayerControllerRef` _asbp_player_controller _stampminigameref)
    (`/Game/Features/Stamping/ToPlace/BP_StampMinigame.Event PossesMinigame` _stampminigameref Interactor)))

(fn `GetActor`
  (returns (Actor :type "Actor Object Reference"))
  (return self))

(fn `IsInteracted`
  (params (value :type Boolean) (player :type "/Game/Players/BP_PlayerCharacter Object Reference"))
  (bind _output_get (set `self.Interacted` value))
  (set `/Game/Players/BP_PlayerCharacter.InteractedWithMinigame` _output_get player))

(fn `UserConstructionScript`)