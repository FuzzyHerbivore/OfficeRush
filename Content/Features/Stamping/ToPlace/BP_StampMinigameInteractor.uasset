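; Pawn a player possesses to play the stamping minigame, after an authorization token check that caches their previous pawn and swaps input mappings.
; Clamped camera look aims sphere traces that highlight items, pick up stamps and papers, or press the reset button; Interact triggers the held stamp.
; Tick returns fallen items to their spawns, and incorrect stamps pulse a post-process glitch.
; Canceling restores the cached pawn and restarts the minigame.
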(event `self.ReceiveBeginPlay`
  (set `self.InitialCameraRotation` (`SceneComponent.K2_GetComponentRotation` (`self.Camera`)))
  ; Post Process Setup
  (set `self.CameraOriginalRotation` (`SceneComponent.K2_GetComponentRotation` (`self.Camera`)))
  (for _array_element (`/Game/Features/Stamping/ToPlace/BP_StampMinigame.StampList` (`self.StampMinigameRef`))
    (add `/Game/Features/Stamping/ToPlace/BP_Stamp.OnStampIncorrect` _array_element (delegate `HandleStampIncorrect`)))
  (bind _returnvalue (`KismetMaterialLibrary.CreateDynamicMaterialInstance` "/Game/Vfx/Materials/M_VFX_PP_Shocked.M_VFX_PP_Shocked"))
  (bind _output_get (set `self.Dynamic Glitch Material` _returnvalue))
  (set `CameraComponent.PostProcessSettings` (make `PostProcessSettings` :`WeightedBlendables` (make `WeightedBlendables` (`|MakeArray` (make `WeightedBlendable` 1.0 _output_get)))) (`self.Camera`)))

(event `HandleStampIncorrect`
  (params (FailedPlayer :type "/Game/Features/Stamping/ToPlace/BP_StampMinigameInteractor Object Reference"))
  ; Post Process Intensity
  (if (== FailedPlayer self)
    (bind (_direction _blend_weight) (`Timeline|Timeline` :!via `PlayFromStart`)
      (:`Update`
        (`MaterialInstanceDynamic.SetScalarParameterValue` (`self.Dynamic Glitch Material`) "Intensity" _blend_weight)))))

(event `EnhancedInput|/Game/UX/IA_Canceling`
  (params (ActionValue :type Boolean) (ElapsedSeconds :type "Float (double-precision)") (TriggeredSeconds :type "Float (double-precision)") (InputAction :type "InputAction Object Reference" :default "/Game/UX/IA_Canceling.IA_Canceling"))
  ; Exit Minigame
  (:`Triggered`
    (`self.ExitMinigame`)))

(event `Event Possess Interactor`
  (params (Interactor :type "Actor Object Reference"))
  (bind _stampminigameref (`self.StampMinigameRef`))
  (bind (_authorizedtokens_datatable _authorizedtokens_rowname) (break `DataTableRowHandle` (`/Game/Features/Stamping/ToPlace/BP_StampMinigame.AuthorizedTokens` (`self.StampMinigameRef`))))
  (bind _returnvalue (pcsubsystem `EnhancedInputLocalPlayerSubsystem` (`/Game/Features/Stamping/ToPlace/BP_StampMinigame.PlayerControllerRef` (`self.StampMinigameRef`))))
  ; Take control of this pawn if authorized
  (bind _asbpi_authorizer (cast `/Game/Libraries/Authorization/BPI_Authorizer` Interactor))
  (bind _returnvalue_2 (`|GetDataTableRow` "/Game/Libraries/Authorization/DT_AuthorizationTokens.DT_AuthorizationTokens" _authorizedtokens_rowname)
    (:`then`
      (bind _isauthorized (`/Game/Libraries/Authorization/BPI_Authorizer.CheckAuthorization` _asbpi_authorizer (`|MakeArray` _returnvalue_2)))
      (if _isauthorized
        (`|ExecutionSequence`
          (:`then_0`
            ; Cache the previous Pawn
            (bind _aspawn (cast `Pawn` Interactor))
            (bind _asbpi_cache (cast `/Game/Libraries/Cache/BPI_Cache` (`self.GetController` _aspawn)))
            (`/Game/Libraries/Cache/BPI_Cache.Cache` _asbpi_cache Interactor))
          (:`then_1`
            (bind _asbpi_controller (cast `/Game/Libraries/Controlling/BPI_Controller` Interactor))
            (`/Game/Libraries/Controlling/BPI_Controller.TakeControl` _asbpi_controller self)
            (`EnhancedInputSubsystemInterface.AddMappingContext` _returnvalue "/Game/Input/IMC_Tasks.IMC_Tasks" 0 (struct))
            (`EnhancedInputSubsystemInterface.RemoveMappingContext` _returnvalue "/Game/Input/IMC_Default.IMC_Default" (struct))
            (`self.SetPlayerPosition`)
            (set `/Game/Features/Stamping/ToPlace/BP_StampDesk.Interacted` true (`/Game/Features/Stamping/ToPlace/BP_StampMinigame.StampDesk` (`self.StampMinigameRef`)))
            (`/Game/Players/BP_PlayerController.OnMinigameEnteredOnce` (`/Game/Features/Stamping/ToPlace/BP_StampMinigame.PlayerControllerRef` (`self.StampMinigameRef`)) 0)
            (`/Game/Players/BP_PlayerCharacter.Event MinigameEntered` (`/Game/Features/Stamping/ToPlace/BP_StampMinigame.PlayerCharacterRef` (`self.StampMinigameRef`)))))
        (else
          (`GameplayStatics.PlaySoundAtLocation` "/Game/SoundAndMusic/SoundEffects/InteractionSounds/MS_InteractionFail.MS_InteractionFail" (`self.K2_GetActorLocation`) (struct) 1.0 1.0 0.0 null null null null)
          (`PlayerController.PlayDynamicForceFeedback` (`/Game/Features/Stamping/ToPlace/BP_StampMinigame.PlayerControllerRef` _stampminigameref) (`/Game/Features/Stamping/ToPlace/BP_StampMinigame.VibrationIntensity` _stampminigameref) (`/Game/Features/Stamping/ToPlace/BP_StampMinigame.NoAuthorizationVibrationDuration` _stampminigameref) true true true true))))))

(event `EnhancedInput|/Game/Input/Actions/IA_Look`
  (params (ActionValue :type "Vector2D Structure") (ElapsedSeconds :type "Float (double-precision)") (TriggeredSeconds :type "Float (double-precision)") (InputAction :type "InputAction Object Reference" :default "/Game/Input/Actions/IA_Look.IA_Look"))
  (bind _returnvalue (`GameplayStatics.GetWorldDeltaSeconds`))
  (bind _camera (`self.Camera`))
  (bind (_initialcamerarotation_roll _initialcamerarotation_pitch _initialcamerarotation_yaw) (`KismetMathLibrary.BreakRotator` (`self.InitialCameraRotation`)))
  (bind _returnvalue_2 (`SceneComponent.K2_GetComponentLocation` _camera))
  (bind (_relativerotation_roll _relativerotation_pitch _relativerotation_yaw) (`KismetMathLibrary.BreakRotator` (`SceneComponent.RelativeRotation` (`self.Camera`))))
  ; Move Camera
  (:`Triggered`
    (bind _output (`self.ClampCameraYaw` (+ (* (* ActionValue_X _returnvalue) (`self.CameraLookSpeed`)) _relativerotation_yaw) _initialcamerarotation_yaw (`self.CameraHorizontalRange`)))
    (bind _output_2 (`self.ClampCameraPitch` (+ (* (* ActionValue_Y _returnvalue) -1.0 (`self.CameraLookSpeed`)) _relativerotation_pitch) _initialcamerarotation_pitch (`self.CameraVerticalRange`)))
    (`SceneComponent.K2_SetRelativeRotation` (`self.Camera`) (`KismetMathLibrary.MakeRotator` 0.0 _output_2 _output) false false)
    (`KismetSystemLibrary.DrawDebugLine` _returnvalue_2 (+ _returnvalue_2 (`SceneComponent.K2_GetComponentRotation` _camera) (* (`SceneComponent.GetForwardVector` _camera) 1000)) (struct :`R` 1.0 :`B` 0.027297 :`A` 1.0) 0.1 0.1)))

(event `self.ReceiveTick`
  (params (DeltaSeconds :type "Float (single-precision)"))
  (bind _camera (`self.Camera`))
  (bind _camera_2 (`self.Camera`))
  (bind _lasthoveredactor (`self.LastHoveredActor`))
  (bind _stampminigameref (`self.StampMinigameRef`))
  (bind _returnvalue (`SceneComponent.K2_GetComponentLocation` _camera_2))
  (bind _paperspawnlocation (`/Game/Features/Stamping/ToPlace/BP_StampMinigame.PaperSpawnLocation` _stampminigameref))
  (bind _paper (`/Game/Features/Stamping/BP_StampPaper.Paper` (`/Game/Features/Stamping/ToPlace/BP_StampMinigame.CurrentPaperRef` _stampminigameref)))
  (bind (_returnvalue_x _returnvalue_y _returnvalue_z) (`KismetMathLibrary.BreakVector` (`SceneComponent.K2_GetComponentLocation` (`/Game/Features/Stamping/ToPlace/BP_StampDesk.ItemResetHeight` (`/Game/Features/Stamping/ToPlace/BP_StampMinigame.StampDesk` (`self.StampMinigameRef`))))))
  (bind (_returnvalue_x_2 _returnvalue_y_2 _returnvalue_z_2) (`KismetMathLibrary.BreakVector` (`SceneComponent.K2_GetComponentLocation` (`/Game/Features/Stamping/BP_StampPaper.Paper` (`/Game/Features/Stamping/ToPlace/BP_StampMinigame.CurrentPaperRef` (`self.StampMinigameRef`))))))
  ; Item Pickup
  (`|ExecutionSequence`
    (:`then_0`
      ; Reset Stamps if Out of Bounds
      (for _array_element (`/Game/Features/Stamping/ToPlace/BP_StampMinigame.StampList` (`self.StampMinigameRef`))
        (bind _out (`self.CheckIfOutOfBounds` _array_element))
        (if _out
          (for _array_element_2 (`/Game/Features/Stamping/ToPlace/BP_StampMinigame.StampStruct` (`self.StampMinigameRef`))
            (if (== (break `/Game/Features/Stamping/F_StampStruct` _array_element_2) _array_element)
              (bind _cube (`/Game/Features/Stamping/ToPlace/BP_Stamp.Cube` _array_element))
              (`SceneComponent.K2_SetWorldLocation` _cube (`.StampOriginalLocation_8_75D2DABD461480A83E73B3B034B73482` (break `/Game/Features/Stamping/F_StampStruct` _array_element_2)) false false)
              (`SceneComponent.K2_SetWorldRotation` _cube (`.StampOriginalRotation_10_8BD41FB4436997E0163873ABB64E9C77` (break `/Game/Features/Stamping/F_StampStruct` _array_element_2)) false false)
              (`PrimitiveComponent.SetPhysicsLinearVelocity` _cube (0.0 0.0 0.0) false "None"))))))
    (:`then_1`
      (if (<= _returnvalue_z_2 _returnvalue_z)
        (`SceneComponent.K2_SetWorldLocation` _paper (`SceneComponent.K2_GetComponentLocation` _paperspawnlocation) false false)
        (`SceneComponent.K2_SetWorldRotation` _paper (`SceneComponent.K2_GetComponentRotation` _paperspawnlocation) false false)
        (`PrimitiveComponent.SetPhysicsLinearVelocity` _paper (0.0 0.0 0.0) false "None")))
    (:`then_2`
      (if (stale `Event Pickup` _output_get_2)
        (message `/Game/Libraries/Minigames/BPI_MinigameInteractable.MinigameInteractedContinous` (`self.SelectedObject`) null (`SceneComponent.K2_GetComponentLocation` _camera) (`KismetMathLibrary.Conv_RotatorToVector` (`SceneComponent.K2_GetComponentRotation` _camera)) (* (`SceneComponent.GetForwardVector` _camera) (`self.HoldDistanceFromCamera`)))
        (else
          ; Outline
          (if (`/Game/Features/Stamping/ToPlace/BP_StampDesk.Interacted` (`/Game/Features/Stamping/ToPlace/BP_StampMinigame.StampDesk` (`self.StampMinigameRef`)))
            (bind _outhit (`KismetSystemLibrary.SphereTraceSingle` :`Start` _returnvalue :`End` (+ _returnvalue (`SceneComponent.K2_GetComponentRotation` _camera_2) (* (`SceneComponent.GetForwardVector` _camera_2) 1000)) :`Radius` 0.5 :`TraceChannel` "TraceTypeQuery1" :`DrawDebugType` "ForDuration" :`DrawTime` 0.1))
            (bind (_bblockinghit _binitialoverlap _time _distance _location _impactpoint _normal _impactnormal _physmat _hitactor) (`GameplayStatics.BreakHitResult` _outhit))
            (if (!= _hitactor _lasthoveredactor)
              (`|ExecutionSequence`
                (:`then_0`
                  (`/Engine/EditorBlueprintResources/StandardMacros.IsValid` _lasthoveredactor
                    (:`Is Valid`
                      (message `/Game/Features/Stamping/BPI_Hoverable.Hovered` _lasthoveredactor false))))
                (:`then_1`
                  (`/Engine/EditorBlueprintResources/StandardMacros.IsValid` _hitactor
                    (:`Is Valid`
                      (message `/Game/Features/Stamping/BPI_Hoverable.Hovered` _hitactor true))))
                (:`then_2`
                  (set `self.LastHoveredActor` _hitactor))))))))))

(event `Event Pickup`
  (bind _camera (`self.Camera`))
  (bind _returnvalue (`SceneComponent.K2_GetComponentLocation` _camera))
  ; Item Pickup
  (if (`self.IsInteracting`) :!label _label
    (message `/Game/Libraries/Minigames/BPI_MinigameInteractable.MinigameInteractedEnded` (`self.SelectedObject`) null (0.0 0.0 0.0) (0.0 0.0 0.0) (0.0 0.0 0.0))
    (set `self.SelectedObject` null)
    (set `self.IsInteracting` false)
    (else
      (bind _outhit (`KismetSystemLibrary.SphereTraceSingle` :`Start` _returnvalue :`End` (+ _returnvalue (`SceneComponent.K2_GetComponentRotation` _camera) (* (`SceneComponent.GetForwardVector` _camera) 1000)) :`Radius` 0.5 :`TraceChannel` "TraceTypeQuery1" :`DrawDebugType` "ForDuration" :`DrawTime` 1.0))
      (bind (_bblockinghit _binitialoverlap _time _distance _location _impactpoint _normal _impactnormal _physmat _hitactor) (`GameplayStatics.BreakHitResult` _outhit))
      (bind _asbp_stamp_minigame_reset_button (cast `/Game/Features/Stamping/ToPlace/BP_StampMinigameResetButton` _hitactor)
        (:`then`
          (message `/Game/Libraries/Minigames/BPI_MinigameInteractable.MinigameInteractedStart` _asbp_stamp_minigame_reset_button null (0.0 0.0 0.0) (0.0 0.0 0.0) (0.0 0.0 0.0)))
        (:`CastFailed`
          (bind _asbp_stamp_paper (cast `/Game/Features/Stamping/BP_StampPaper` _hitactor)
            (:`then`
              (if (== (`/Game/Features/Stamping/BP_StampPaper.MarkForFinished` _asbp_stamp_paper) true)
                (if (== (`/Game/Features/Stamping/BP_StampPaper.IsFinished` _asbp_stamp_paper) false)
                  (if (`KismetSystemLibrary.DoesImplementInterface` _hitactor "/Game/Libraries/Minigames/BPI_MinigameInteractable.BPI_MinigameInteractable_C") :!label _label_2
                    (bind _output_get (set `self.SelectedObject` _hitactor))
                    (message `/Game/Libraries/Minigames/BPI_MinigameInteractable.MinigameInteractedStart` _output_get null (0.0 0.0 0.0) (0.0 0.0 0.0) (0.0 0.0 0.0))
                    (bind _output_get_2 (set `self.IsInteracting` true))))))
            (:`CastFailed`
              (goto _label_2))))))))

(event `EnhancedInput|/Game/Input/Actions/IA_Pickup`
  (params (ActionValue :type Boolean) (ElapsedSeconds :type "Float (double-precision)") (TriggeredSeconds :type "Float (double-precision)") (InputAction :type "InputAction Object Reference" :default "/Game/Input/Actions/IA_Pickup.IA_Pickup"))
  ; Item Pickup
  (:`Started`
    (goto _label)))

(event `EnhancedInput|/Game/Input/Actions/IA_Interact`
  (params (ActionValue :type Boolean) (ElapsedSeconds :type "Float (double-precision)") (TriggeredSeconds :type "Float (double-precision)") (InputAction :type "InputAction Object Reference" :default "/Game/Input/Actions/IA_Interact.IA_Interact"))
  ; Stamp Action
  (:`Started`
    (if (`self.IsInteracting`)
      (bind _asbp_stamp (cast `/Game/Features/Stamping/ToPlace/BP_Stamp` (`self.SelectedObject`)))
      (`/Game/Features/Stamping/ToPlace/BP_Stamp.Event BeginStamp` _asbp_stamp))))

(fn `CheckIfOutOfBounds`
  (params (Actor :type "Actor Object Reference"))
  (returns (out :type Boolean))
  (bind (_returnvalue_x _returnvalue_y _returnvalue_z) (`KismetMathLibrary.BreakVector` (`self.K2_GetActorLocation` Actor)))
  (bind (_returnvalue_x_2 _returnvalue_y_2 _returnvalue_z_2) (`KismetMathLibrary.BreakVector` (`SceneComponent.K2_GetComponentLocation` (`/Game/Features/Stamping/ToPlace/BP_StampDesk.ItemResetHeight` (`/Game/Features/Stamping/ToPlace/BP_StampMinigame.StampDesk` (`self.StampMinigameRef`))))))
  (return (<= _returnvalue_z _returnvalue_z_2)))

(fn `ClampCameraPitch`
  (params (Value :type "Float (double-precision)") (Axis :type "Float (double-precision)") (RangeValue :type "Vector2D Structure"))
  (returns (output :type "Float (double-precision)"))
  (return (`KismetMathLibrary.FClamp` Value (- Axis RangeValue_X) (+ Axis RangeValue_Y))))

(fn `ClampCameraYaw`
  (params (Value :type "Float (double-precision)") (Axis :type "Float (double-precision)") (RangeValue :type "Vector2D Structure"))
  (returns (output :type "Float (double-precision)"))
  (bind (_returnvalue_roll _returnvalue_pitch _returnvalue_yaw) (`KismetMathLibrary.BreakRotator` (`KismetMathLibrary.NormalizedDeltaRotator` (`KismetMathLibrary.MakeRotator` 0.0 0.0 Value) (`KismetMathLibrary.MakeRotator` 0.0 0.0 Axis))))
  (return (+ (`KismetMathLibrary.FClamp` _returnvalue_yaw (* RangeValue_X -1.0) RangeValue_Y) Axis)))

(fn `ExitMinigame`
  (bind _returnvalue (`self.GetController`))
  (bind _stampminigameref (`self.StampMinigameRef`))
  (bind _playercontrollerref (`/Game/Features/Stamping/ToPlace/BP_StampMinigame.PlayerControllerRef` (`self.StampMinigameRef`)))
  (bind _returnvalue_2 (pcsubsystem `EnhancedInputLocalPlayerSubsystem` (`/Game/Features/Stamping/ToPlace/BP_StampMinigame.PlayerControllerRef` (`self.StampMinigameRef`))))
  (message `/Game/Libraries/Minigames/BPI_MinigameInteractable.MinigameInteractedEnded` (`self.SelectedObject`) null (0.0 0.0 0.0) (0.0 0.0 0.0) (0.0 0.0 0.0))
  (set `self.SelectedObject` null)
  (set `self.IsInteracting` false)
  (bind _asbpi_cache (cast `/Game/Libraries/Cache/BPI_Cache` _returnvalue))
  (bind _actor (`/Game/Libraries/Cache/BPI_Cache.Retrieve` _asbpi_cache))
  (bind _aspawn (cast `Pawn` _actor))
  (`Controller.Possess` _returnvalue _aspawn)
  (`EnhancedInputSubsystemInterface.AddMappingContext` _returnvalue_2 "/Game/Input/IMC_Default.IMC_Default" 0 (struct))
  (`EnhancedInputSubsystemInterface.RemoveMappingContext` _returnvalue_2 "/Game/Input/IMC_Tasks.IMC_Tasks" (struct))
  (set `/Game/Features/Stamping/ToPlace/BP_StampDesk.Interacted` false (`/Game/Features/Stamping/ToPlace/BP_StampMinigame.StampDesk` _stampminigameref))
  (`/Game/Features/Stamping/ToPlace/BP_StampMinigame.RestartMinigame` _stampminigameref)
  (`/Game/Players/BP_PlayerController.OnTaskCompletedOnce` _playercontrollerref (`GameplayStatics.GetPlayerControllerID` _playercontrollerref))
  (`/Game/Players/BP_PlayerCharacter.Event MinigameExited` (`/Game/Features/Stamping/ToPlace/BP_StampMinigame.PlayerCharacterRef` (`self.StampMinigameRef`))))

(fn `ResetCameraRotation`
  (`SceneComponent.K2_SetWorldRotation` (`self.Camera`) (`self.CameraOriginalRotation`) false false))

(fn `SetPlayerPosition`
  (bind _stampminigameref (`self.StampMinigameRef`))
  (bind _playerstandlocation (`/Game/Features/Stamping/ToPlace/BP_StampMinigame.PlayerStandLocation` _stampminigameref))
  (`self.K2_SetActorLocationAndRotation` (`/Game/Features/Stamping/ToPlace/BP_StampMinigame.PlayerCharacterRef` _stampminigameref) (`SceneComponent.K2_GetComponentLocation` _playerstandlocation) (`SceneComponent.K2_GetComponentRotation` _playerstandlocation) false true))

(fn `UserConstructionScript`)