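; BP_Task is a task actor that acts as a collectable, exposing its icon, name, category, color and collection behavior.
; SetTaskData stores the TaskData struct that drives every getter.
; Color and authorization token resolve through row references into DT_TaskColors and DT_AuthorizationTokens, while the other values come straight from the struct.
; Collect and drop events are empty, and OnReset destroys the actor.
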(event `/Game/Libraries/Inventory/BPI_Collectable.OnCollected`)

(event `/Game/Libraries/Inventory/BPI_Collectable.OnDropped`
  (params (Location :type "Vector Structure")))

(event `/Game/Libraries/Inventory/BPI_Collectable.OnReset`
  (`self.K2_DestroyActor`))

(fn `GetAuthorizationToken`
  (returns (AuthorizationToken :type "/Game/Libraries/Authorization/S_AuthorizationToken Structure"))
  (bind _returnvalue (`|GetDataTableRow` "/Game/Libraries/Authorization/DT_AuthorizationTokens.DT_AuthorizationTokens" (`.RowName` (break `DataTableRowHandle` (`.AuthorizationTokensRow_21_7622A1B6495432E83D6BA19D5D1AD17E` (break `/Game/Features/Tasks/S_TaskData` (`self.TaskData`))))))
    (:`then`
      (return _returnvalue))))

(fn `GetCollactableIcon`
  (returns (Icon :type "SlateBrushAsset Object Reference"))
  (bind (_taskdata_name _taskdata_symboltexturediffuse _taskdata_symboltextureemission _taskdata_taskcolorsrow _taskdata_uiicon) (break `/Game/Features/Tasks/S_TaskData` (`self.TaskData`)))
  (return _taskdata_uiicon))

(fn `GetCollectableCategory`
  (returns (Category :type String))
  (bind (_taskdata_name _taskdata_symboltexturediffuse _taskdata_symboltextureemission _taskdata_taskcolorsrow _taskdata_uiicon _taskdata_authorizationtokensrow _taskdata_collectablecategory) (break `/Game/Features/Tasks/S_TaskData` (`self.TaskData`)))
  (return _taskdata_collectablecategory))

(fn `GetCollectableColor`
  (returns (ColorCurveValue :type "Float (double-precision)"))
  (bind (_taskdata_name _taskdata_symboltexturediffuse _taskdata_symboltextureemission _taskdata_taskcolorsrow) (break `/Game/Features/Tasks/S_TaskData` (`self.TaskData`)))
  (bind _returnvalue (`|GetDataTableRow` "/Game/Features/Tasks/DT_TaskColors.DT_TaskColors" (`.RowName` (break `DataTableRowHandle` _taskdata_taskcolorsrow)))
    (:`then`
      (return (`.ColorCurveValue_2_55EE6E1545189B47A3B901980D1ED714` (break `/Game/Features/Tasks/S_TaskColor` _returnvalue))))))

(fn `GetCollectableName`
  (returns (Name :type String))
  (bind _taskdata_name (break `/Game/Features/Tasks/S_TaskData` (`self.TaskData`)))
  (return _taskdata_name))

(fn `GetCollectionBehavior`
  (returns (CollectionBehavior :type "/Game/Libraries/Inventory/E_CollectionBehavior Enum"))
  (bind (_taskdata_name _taskdata_symboltexturediffuse _taskdata_symboltextureemission _taskdata_taskcolorsrow _taskdata_uiicon _taskdata_authorizationtokensrow _taskdata_collectablecategory _taskdata_collectionbehavior) (break `/Game/Features/Tasks/S_TaskData` (`self.TaskData`)))
  (return _taskdata_collectionbehavior))

(fn `SetTaskData`
  (params (TaskDataToSet :type "/Game/Features/Tasks/S_TaskData Structure"))
  (set `self.TaskData` TaskDataToSet))

(fn `UserConstructionScript`)