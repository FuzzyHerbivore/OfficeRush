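; Interactable task board that shows a queue of random tasks and hands the oldest to the interacting player.
; Child BP_TaskListSlot actors display the queue, which refills from a data table with an optional duplicate limit.
; Interact plays pickup FX, then after a delay spawns a BP_Task for BPI_Inventory, advancing the queue if collected or destroying it otherwise.
; Focus highlights the top-priority slot, and new-task sounds skip the initial fill.
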(event `self.ReceiveBeginPlay`
  (for _array_element (`self.GetAllChildActors` false)
    (bind _asbp_task_list_slot (cast `/Game/Features/Tasks/BP_TaskListSlot` _array_element))
    (`KismetArrayLibrary.Array_Add` (`self.TaskListSlots`) _asbp_task_list_slot))
  (`self.FillTaskDataList`)
  (`self.TaskListUpdated`)
  (set `self.SoundShouldPlay` true))

(event `TaskListUpdated`
  (for (_array_element _array_index) (`self.TaskListSlots`)
    (`/Game/Features/Tasks/BP_TaskListSlot.SetTaskData` _array_element (`|GetArrayItem` (`self.TaskDataList`) _array_index))
    (if (`self.SoundShouldPlay`)
      (`GameplayStatics.PlaySoundAtLocation` "/Game/SoundAndMusic/SoundEffects/SystemNotificationSounds/MS_NewTask.MS_NewTask" (`self.K2_GetActorLocation`) (struct) 1.0 1.0 0.0 null null null null))))

(event `/Game/Libraries/Interaction/BPI_Interactable.Interact`
  (params (Interactor :type "Actor Object Reference (by ref)"))
  (`|ExecutionSequence`
    (:`then_0`
      (if (`self.SoundShouldPlay`)
        (`ActorComponent.Activate` (`/Game/Features/Tasks/BP_TaskListSlot.FXS_VFX_PickUp` (`|GetArrayItem` (`self.TaskListSlots`))) false)))
    (:`then_1`
      (`KismetSystemLibrary.Delay` 0.8)
      (bind _taskdata (`self.GetOldestTaskDataFromList`))
      (bind _returnvalue (`|SpawnActorFromClass` "/Game/Features/Tasks/BP_Task.BP_Task_C" (`self.GetTransform`) "Undefined" "MultiplyWithRoot" null null))
      (`/Game/Features/Tasks/BP_Task.SetTaskData` _returnvalue _taskdata)
      (bind _asbpi_inventory (cast `/Game/Libraries/Inventory/BPI_Inventory` Interactor)
        (:`then`
          (bind _wassuccessful (`/Game/Libraries/Inventory/BPI_Inventory.Collect` _asbpi_inventory _returnvalue))
          (if _wassuccessful
            (`self.RemoveOldestTaskDataFromList`)
            (`KismetSystemLibrary.Delay` (`self.TaskAcceptSoundDelay`))
            (`GameplayStatics.PlaySound2D` "/Game/SoundAndMusic/SoundEffects/SystemNotificationSounds/MS_TaskAccept.MS_TaskAccept" 1.0 1.0 0.0 null null)
            (else
              (`self.K2_DestroyActor` _returnvalue :!label _label))))
        (:`CastFailed`
          (goto _label))))))

(event `/Game/Libraries/Interaction/BPI_Interactable.Focus`
  (params (IsOn :type Boolean))
  (if (not (== IsOn (`self.IsFocused`)))
    (bind _output_get (set `self.IsFocused` IsOn))
    (bind _asbp_task_list_slot (cast `/Game/Features/Tasks/BP_TaskListSlot` (`ChildActorComponent.ChildActor` (`self.BP_TaskListSlotPrio1`))))
    (`/Game/Features/Tasks/BP_TaskListSlot.Focus` _asbp_task_list_slot _output_get)))

(fn `CheckIfOverDuplicateLimit`
  (params (NewData :type "/Game/Features/Tasks/S_TaskData Structure") (ExistingData :type "Array of /Game/Features/Tasks/S_TaskData Structure"))
  (returns (IsWithinLimit :type Boolean))
  (locals (AmountDuplicates :type Integer) (NewLocalVar :type String))
  (if (== (`self.AmountLimitOfDuplicates`) 0)
    (return true)
    (else
      (for _array_element ExistingData
        (if (`KismetStringLibrary.EqualEqual_StrStr` (`.Name_2_36BE8D9D4CED24DFDBBCC99F79F273F5` (break `/Game/Features/Tasks/S_TaskData` _array_element)) (`.Name_2_36BE8D9D4CED24DFDBBCC99F79F273F5` (break `/Game/Features/Tasks/S_TaskData` NewData)))
          (set `local.AmountDuplicates` (+ (`local.AmountDuplicates`) 1))))
      (return (< (`local.AmountDuplicates`) (`self.AmountLimitOfDuplicates`))))))

(fn `FillTaskDataList`
  (bind _taskdatalist (`self.TaskDataList`))
  (while (< (`KismetArrayLibrary.Array_Length` _taskdatalist) (`KismetArrayLibrary.Array_Length` (`self.TaskListSlots`)))
    (bind _taskdata (`self.GetRandomTaskData`))
    (bind _iswithinlimit (`self.CheckIfOverDuplicateLimit` _taskdata _taskdatalist))
    (if _iswithinlimit
      (`KismetArrayLibrary.Array_Add` _taskdatalist _taskdata)))
  (return))

(fn `GetActor`
  (returns (Actor :type "Actor Object Reference"))
  (return self))

(fn `GetOldestTaskDataFromList`
  (returns (TaskData :type "/Game/Features/Tasks/S_TaskData Structure"))
  (return (`|GetArrayItem` (`self.TaskDataList`))))

(fn `GetRandomTaskData`
  (returns (TaskData :type "/Game/Features/Tasks/S_TaskData Structure"))
  (bind _outrownames (`DataTableFunctionLibrary.GetDataTableRowNames` (`self.TaskDataTable`)))
  (bind _returnvalue (`|GetDataTableRow` "/Game/Features/Tasks/DT_Tasks.DT_Tasks" (`KismetArrayLibrary.Array_Random` _outrownames))
    (:`then`
      (return _returnvalue))))

(fn `InitTaskListSlots`
  (locals (TaskListSlotss :type "Array of /Game/Features/Tasks/BP_TaskListSlot Object Reference"))
  (for _array_element (`self.GetAllChildActors` false)
    (bind _asbp_task_list_slot (cast `/Game/Features/Tasks/BP_TaskListSlot` _array_element))
    (`KismetArrayLibrary.Array_Add` (`self.TaskListSlots`) _asbp_task_list_slot))
  (return))

(fn `RemoveOldestTaskDataFromList`
  (locals (TaskDataToReturn :type "/Game/Features/Tasks/S_TaskData Structure"))
  (`KismetArrayLibrary.Array_Remove` (`self.TaskDataList`))
  (`self.FillTaskDataList`)
  (`self.TaskListUpdated`)
  (return))

(fn `UserConstructionScript`)