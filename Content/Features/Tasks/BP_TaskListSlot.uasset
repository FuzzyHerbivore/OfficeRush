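; BP_TaskListSlot is a task list slot that displays a task's symbol and color and reacts to focus.
; SetTaskData stores the task and triggers TaskDataUpdated, which uses its DT_TaskColors row and symbol textures to rebuild the slot's dynamic material.
; One color curve value drives both material LUT parameters and the tint of the selection and pickup Niagara effects.
; Focus toggles the selection effect and animates the material's HoverLerp through timelines.
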(event `self.ReceiveBeginPlay`
  (`ActorComponent.Deactivate` (`self.FXS_VFX_Selection_01`))
  (`ActorComponent.Deactivate` (`self.FXS_VFX_PickUp`)))

(event `TaskDataUpdated`
  (bind _dynamicmaterialinstance (`self.DynamicMaterialInstance`))
  (bind _taskdata (`self.TaskData`))
  (bind _returnvalue (`|GetDataTableRow` "/Game/Features/Tasks/DT_TaskColors.DT_TaskColors" (`.RowName` (break `DataTableRowHandle` (`.TaskColorsRow_31_801F51CB40708504EED085BE48C868F7` (break `/Game/Features/Tasks/S_TaskData` _taskdata)))))
    (:`then`
      (bind _returnvalue_2 (`PrimitiveComponent.CreateDynamicMaterialInstance` (`self.Slot`) 0 "/Game/Environment/Assets/Taskboard/M_Inst_Task_Base.M_Inst_Task_Base" "None"))
      (bind _output_get (set `self.DynamicMaterialInstance` _returnvalue_2))
      (bind _colorcurvevalue (break `/Game/Features/Tasks/S_TaskColor` _returnvalue))
      (`MaterialInstanceDynamic.SetScalarParameterValue` _output_get "TintColor LUT" _colorcurvevalue)
      (`MaterialInstanceDynamic.SetScalarParameterValue` _dynamicmaterialinstance "EmissiveColor LUT" _colorcurvevalue)
      (`MaterialInstanceDynamic.SetTextureParameterValue` _dynamicmaterialinstance "Diffuse" (`.SymbolTextureDiffuse_37_69F45A654475D649F0A634A0BD659943` (break `/Game/Features/Tasks/S_TaskData` _taskdata)))
      (`MaterialInstanceDynamic.SetTextureParameterValue` _dynamicmaterialinstance "Emissive Mask" (`.SymbolTextureEmission_40_3D93E8014207496C71EDAD90693BC072` (break `/Game/Features/Tasks/S_TaskData` _taskdata)))
      (`NiagaraComponent.SetNiagaraVariableFloat` (`self.FXS_VFX_Selection_01`) "User_ParticleColor" _colorcurvevalue)
      (`NiagaraComponent.SetNiagaraVariableFloat` (`self.FXS_VFX_PickUp`) "User_ParticleColor" _colorcurvevalue))))

(event `Focus`
  (params (IsOn :type Boolean))
  (if IsOn
    (`ActorComponent.Activate` (`self.FXS_VFX_Selection_01`) false)
    (bind (_direction _hover_animation) (`Timeline|Timeline` :!via `PlayFromStart`)
      (:`Update`
        (`MaterialInstanceDynamic.SetScalarParameterValue` (`self.DynamicMaterialInstance`) "HoverLerp" _hover_animation)))
    (else
      (`ActorComponent.Deactivate` (`self.FXS_VFX_Selection_01`))
      (bind (_direction_2 _hover_animation_2) (`Timeline|Timeline_0` :!via `ReverseFromEnd`)
        (:`Update`
          (`MaterialInstanceDynamic.SetScalarParameterValue` (`self.DynamicMaterialInstance`) "HoverLerp" _hover_animation_2))))))

(fn `SetTaskData`
  (params (TaskDataToBeSet :type "/Game/Features/Tasks/S_TaskData Structure"))
  (set `self.TaskData` TaskDataToBeSet)
  (`self.TaskDataUpdated`))

(fn `UserConstructionScript`
  (bind _returnvalue (`PrimitiveComponent.CreateDynamicMaterialInstance` (`self.Slot`) 0 "/Game/Environment/Assets/Taskboard/M_Inst_Task_Base.M_Inst_Task_Base" "None"))
  (set `self.DynamicMaterialInstance` _returnvalue))