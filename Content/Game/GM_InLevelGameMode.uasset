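; In-level game mode that sets up local multiplayer for a game with sorting, stamp and email minigames and handles restarts.
; On BeginPlay it spawns a movement-locked character with its own mesh at each player start, creating extra local players, and spawns the UI handler.
; EnableMovement later restores walking.
; RestartGame exits minigames, resets keycards, inventories and scores, then respawns characters without the movement lock and refreshes UI.
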(event `self.ReceiveBeginPlay`
  (`|ExecutionSequence`
    (:`then_0`
      (bind _outactors (`GameplayStatics.GetAllActorsOfClass` "/Game/Players/BP_PlayerStart.BP_PlayerStart_C"))
      (for (_array_element _array_index) _outactors
        (bind _charactermesh (`/Game/Players/BP_PlayerStart.GetCharacterMesh` _array_element))
        (if (>= _array_index 1)
          (bind _returnvalue (`GameplayStatics.CreatePlayer` _array_index))
          (set `self.ControllerToPossessPawnWith` _returnvalue)
          (else
            (set `self.ControllerToPossessPawnWith` (`GameplayStatics.GetPlayerController` 0))))
        (bind _returnvalue_2 (`|SpawnActorFromClass` "/Game/Players/BP_PlayerCharacter.BP_PlayerCharacter_C" (`self.GetTransform` _array_element) "Undefined" "MultiplyWithRoot" null null))
        (`SkeletalMeshComponent.SetSkeletalMeshAsset` (`Character.Mesh` _returnvalue_2) _charactermesh)
        (`Controller.Possess` (`self.ControllerToPossessPawnWith`) _returnvalue_2)
        (`CharacterMovementComponent.DisableMovement` (`Character.CharacterMovement` _returnvalue_2))))
    (:`then_1`
      (`|SpawnActorFromClass` "/Game/UI/UIHandle/BP_UIHandler.BP_UIHandler_C" (`KismetMathLibrary.Conv_VectorToTransform` (0.0 0.0 0.0)) "AlwaysSpawn" "MultiplyWithRoot" null null))
    (:`then_2`
      (add `self.RestartingGame` (delegate `RestartGame`)))))

(event `EnableMovement`
  (bind _outactors (`GameplayStatics.GetAllActorsOfClass` "/Game/Players/BP_PlayerController.BP_PlayerController_C"))
  (for _array_element _outactors
    (bind _asbp_player_character (cast `/Game/Players/BP_PlayerCharacter` (`Controller.K2_GetPawn` _array_element)))
    (`CharacterMovementComponent.SetMovementMode` (`Character.CharacterMovement` _asbp_player_character) "MOVE_Walking" 0)))

(event `RestartGame`
  (bind _returnvalue (`GameplayStatics.GetActorOfClass` "/Game/Features/PaperSorting/BP_SortingMinigameInteractor.BP_SortingMinigameInteractor_C"))
  (`/Game/Features/PaperSorting/BP_SortingMinigameInteractor.ExitMinigame` _returnvalue)
  (bind _returnvalue_2 (`GameplayStatics.GetActorOfClass` "/Game/Features/Stamping/ToPlace/BP_StampMinigameInteractor.BP_StampMinigameInteractor_C"))
  (`/Game/Features/Stamping/ToPlace/BP_StampMinigameInteractor.ExitMinigame` _returnvalue_2)
  (bind _outactors (`GameplayStatics.GetAllActorsOfClass` "/Game/Features/Email/BP_EmailMinigameInteractor.BP_EmailMinigameInteractor_C"))
  (for _array_element _outactors
    (`/Game/Features/Email/BP_EmailMinigameInteractor.ExitMinigame` _array_element)
    (bind _outactors_2 (`GameplayStatics.GetAllActorsOfClass` "/Game/Features/Doors/BP_Keycard.BP_Keycard_C"))
    (for _array_element_2 _outactors_2
      (`/Game/Features/Doors/BP_Keycard.OnGameRestartedNotifyKeycard` _array_element_2)))
  (bind _outactors_3 (`GameplayStatics.GetAllActorsOfClass` "/Game/Players/BP_PlayerController.BP_PlayerController_C"))
  (for _array_element_3 _outactors_3
    ; Unpossesing and resetting Variables
    (`EnhancedInputLibrary.FlushPlayerInput` _array_element_3)
    (bind _output_get (set `self.CharToDestroy` (`Controller.K2_GetPawn` _array_element_3)))
    (bind _asbpi_inventory (cast `/Game/Libraries/Inventory/BPI_Inventory` _output_get))
    (`/Game/Libraries/Inventory/BPI_Inventory.RemoveAllCollectables` _asbpi_inventory)
    (`Controller.UnPossess` _array_element_3)
    (`self.K2_DestroyActor` _output_get)
    (set `/Game/Players/BP_PlayerController.Score` 0 _array_element_3))
  ; Spawning Player Character
  (bind _outactors_4 (`GameplayStatics.GetAllActorsOfClass` "/Game/Players/BP_PlayerStart.BP_PlayerStart_C"))
  (for (_array_element_4 _array_index) _outactors_4
    (bind _charactermesh (`/Game/Players/BP_PlayerStart.GetCharacterMesh` _array_element_4))
    (bind _returnvalue_3 (`|SpawnActorFromClass` "/Game/Players/BP_PlayerCharacter.BP_PlayerCharacter_C" (`self.GetTransform` _array_element_4) "Undefined" "MultiplyWithRoot" null null))
    (`SkeletalMeshComponent.SetSkeletalMeshAsset` (`Character.Mesh` _returnvalue_3) _charactermesh)
    (`Controller.Possess` (`GameplayStatics.GetPlayerController` _array_index) _returnvalue_3))
  (bind _returnvalue_4 (`GameplayStatics.GetActorOfClass` "/Game/UI/UIHandle/BP_UIHandler.BP_UIHandler_C"))
  (`/Game/UI/UIHandle/BP_UIHandler.RespawningUI` _returnvalue_4))

(fn `UserConstructionScript`)