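; BP_Interactor lets its owner interact with the closest visible object implementing BPI_Interactable within range.
; InteractionRange overlaps maintain the list of interactables in reach, unfocusing any that leave.
; Each tick it picks the nearest candidate passing a line-of-sight check, focuses it and unfocuses the others.
; InteractWithInteractablesInRange calls Interact on that stored closest target, passing the owner, whenever the list is not empty.
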(event `InteractWithInteractablesInRange`
  (bind _returnvalue (`self.GetOwner`))
  (bind _closestinteractable (`self.ClosestInteractable`))
  (`/Engine/EditorBlueprintResources/StandardMacros.IsValid` _returnvalue
    (:`Is Valid`
      (if (`KismetArrayLibrary.Array_IsEmpty` (`self.InteractablesInReach`))
        _
        (elif (`KismetSystemLibrary.IsValidInterface` _closestinteractable)
          (`/Game/Libraries/Interaction/BPI_Interactable.Interact` _closestinteractable _returnvalue))))))

(event `self.ReceiveTick`
  (params (DeltaSeconds :type "Float (single-precision)"))
  (bind _closestinteractable (`self.ClosestInteractable`))
  (`self.UpdateClosestInteractable`)
  (for _array_element (`self.InteractablesInReach`)
    (if (`KismetSystemLibrary.IsValidInterface` (`self.ClosestInteractable`))
      (bind _actor (`/Game/Libraries/Interaction/BPI_Interactable.GetActor` _array_element))
      (bind _actor_2 (`/Game/Libraries/Interaction/BPI_Interactable.GetActor` _closestinteractable))
      (if (== _actor _actor_2)
        (`/Game/Libraries/Interaction/BPI_Interactable.Focus` _closestinteractable true)
        (else
          (`/Game/Libraries/Interaction/BPI_Interactable.Focus` _array_element false))))))

(event `self.InteractionRange.OnComponentBeginOverlap`
  (params (OverlappedComponent :type "PrimitiveComponent Object Reference") (OtherActor :type "Actor Object Reference") (OtherComp :type "PrimitiveComponent Object Reference") (OtherBodyIndex :type Integer) (bFromSweep :type Boolean) (SweepResult :type "HitResult Structure (by ref)"))
  (bind _asbpi_interactable (cast `/Game/Libraries/Interaction/BPI_Interactable` OtherActor))
  (`KismetArrayLibrary.Array_AddUnique` (`self.InteractablesInReach`) _asbpi_interactable))

(event `self.InteractionRange.OnComponentEndOverlap`
  (params (OverlappedComponent :type "PrimitiveComponent Object Reference") (OtherActor :type "Actor Object Reference") (OtherComp :type "PrimitiveComponent Object Reference") (OtherBodyIndex :type Integer))
  (bind _asbpi_interactable (cast `/Game/Libraries/Interaction/BPI_Interactable` OtherActor))
  (`KismetArrayLibrary.Array_RemoveItem` (`self.InteractablesInReach`) _asbpi_interactable)
  (`/Game/Libraries/Interaction/BPI_Interactable.Focus` _asbpi_interactable false))

(fn `UpdateClosestInteractable`
  (locals (ClosestInteractorDistance :type "Float (double-precision)"))
  (bind _returnvalue (`self.GetOwner`))
  (for (_array_element _array_index) (`self.InteractablesInReach`)
    (bind _actor (`/Game/Libraries/Interaction/BPI_Interactable.GetActor` _array_element))
    (`/Engine/EditorBlueprintResources/StandardMacros.IsValid` _actor
      (:`Is Valid`
        (bind _canseeactorend (`/Game/Libraries/FunctionLibraries/LineOfSight.CanActorStartSeeActorEnd` _returnvalue _actor))
        (if _canseeactorend
          (if (== _array_index 0)
            (bind _returnvalue_2 (`self.GetDistanceTo` _actor _returnvalue))
            (set `local.ClosestInteractorDistance` _returnvalue_2 :!label _label)
            (set `self.ClosestInteractable` _array_element)
            (elif (< _returnvalue_2 (`local.ClosestInteractorDistance`))
              (goto _label)))))
      (:`Is Not Valid`
        (`KismetSystemLibrary.PrintText` (`|FormatText` "Error: {Actor} does not return an Actor when 'GetActor' is called on it!" _actor))))))

(fn `UserConstructionScript`)