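; Inventory component that stores collectables and enforces optional per-category count limits.
; Collect builds an index-to-item map of the incoming item's category and checks it against that category's limit.
; At the limit, the item's collection behavior decides: FIFO resets and evicts the oldest in that category, Block rejects the newcomer.
; Removing one or all collectables also calls OnReset on each removed item.
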(fn `Collect`
  (params (Collectable :type "/Game/Libraries/Inventory/BPI_Collectable Interface"))
  (returns (WasSuccessful :type Boolean))
  (bind _collectables (`self.Collectables`))
  ; Collect collectable, respecting the category limits
  (bind _category (`/Game/Libraries/Inventory/BPI_Collectable.GetCollectableCategory` Collectable))
  (bind _enumeratedcollectablesofcategory (`self.GetCollectablesOfCategory` _category))
  (bind (_value _returnvalue) (`BlueprintMapLibrary.Map_Find` (`self.MaxCountOfCollectablesInCategory`) _category))
  (if _returnvalue
    (if (>= (`BlueprintMapLibrary.Map_Length` _enumeratedcollectablesofcategory) _value)
      (bind _keys (`BlueprintMapLibrary.Map_Keys` _enumeratedcollectablesofcategory))
      (bind _collectionbehavior (`/Game/Libraries/Inventory/BPI_Collectable.GetCollectionBehavior` Collectable))
      (switch `/Game/Libraries/Inventory/E_CollectionBehavior` _collectionbehavior
        (:`NewEnumerator0`
          (bind _output (`|GetArrayItem` _keys))
          (`/Game/Libraries/Inventory/BPI_Collectable.OnReset` (`|GetArrayItem` _collectables _output))
          (`KismetArrayLibrary.Array_Remove` _collectables _output))
        (:`NewEnumerator1`
          (return false)))))
  (`KismetArrayLibrary.Array_Add` (`self.Collectables`) Collectable)
  (return true))

(fn `GetCollectablesOfCategory`
  (params (Category :type String))
  (returns (EnumeratedCollectablesOfCategory :type "Map of Integer to /Game/Libraries/Inventory/BPI_Collectable Interface"))
  (locals (CollectablesOfCategory :type "Map of Integer to /Game/Libraries/Inventory/BPI_Collectable Interface"))
  ; Get collectables of a given category
  (`BlueprintMapLibrary.Map_Clear` (`local.CollectablesOfCategory`))
  (for (_array_element _array_index) (`self.Collectables`)
    (bind _category (`/Game/Libraries/Inventory/BPI_Collectable.GetCollectableCategory` _array_element))
    (if (`KismetStringLibrary.EqualEqual_StrStr` _category Category)
      (`BlueprintMapLibrary.Map_Add` (`local.CollectablesOfCategory`) _array_index _array_element)))
  (return (`local.CollectablesOfCategory`)))

(fn `RemoveAllCollectables`
  (bind (_arrayindex _arrayelement) (`/Engine/EditorBlueprintResources/StandardMacros.ReverseForEachLoop` (`self.Collectables`))
    (:`LoopBody`
      (`self.RemoveCollectable` _arrayelement))))

(fn `RemoveCollectable`
  (params (Collectable :type "/Game/Libraries/Inventory/BPI_Collectable Interface"))
  (returns (WasSuccessful :type Boolean))
  (bind _returnvalue (`KismetArrayLibrary.Array_RemoveItem` (`self.Collectables`) Collectable))
  (`/Game/Libraries/Inventory/BPI_Collectable.OnReset` Collectable)
  (return _returnvalue))