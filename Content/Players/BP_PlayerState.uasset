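; Player state Blueprint that exposes the player's collectable inventory to the rest of the game.
; Each function and the RemoveAllCollectables event forwards directly to the ACInventory component, covering collecting, removing and querying all collectables or those of a given category.
; It holds no inventory logic of its own, acting as a thin facade over that component.
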(event `/Game/Libraries/Inventory/BPI_Inventory.RemoveAllCollectables`
  (`/Game/Libraries/Inventory/BPI_Inventory.RemoveAllCollectables` (`self.AC_Inventory`)))

(fn `Collect`
  (params (Collectable :type "/Game/Libraries/Inventory/BPI_Collectable Interface"))
  (returns (WasSuccessful :type Boolean))
  (bind _wassuccessful (`/Game/Libraries/Inventory/BPI_Inventory.Collect` (`self.AC_Inventory`) Collectable))
  (return _wassuccessful))

(fn `GetAllCollectables`
  (returns (Collectables :type "Array of /Game/Libraries/Inventory/BPI_Collectable Interface"))
  (return (`/Game/Libraries/Inventory/AC_Inventory.Collectables` (`self.AC_Inventory`))))

(fn `GetCollectablesOfCategory`
  (params (Category :type String))
  (returns (CollectablesAtIndex :type "Map of Integer to /Game/Libraries/Inventory/BPI_Collectable Interface"))
  (bind _collectablesatindex (message `/Game/Libraries/Inventory/BPI_Inventory.GetCollectablesOfCategory` (`self.AC_Inventory`) Category))
  (return _collectablesatindex))

(fn `RemoveCollectable`
  (params (Collectable :type "/Game/Libraries/Inventory/BPI_Collectable Interface"))
  (returns (WasSuccessful :type Boolean))
  (bind _wassuccessful (`/Game/Libraries/Inventory/BPI_Inventory.RemoveCollectable` (`self.AC_Inventory`) Collectable))
  (return _wassuccessful))

(fn `UserConstructionScript`)