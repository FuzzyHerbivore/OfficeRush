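; Actor component for BP_NPCharacter that fades a post-process scan effect in and out through StartScanEffect and EndScanEffect.
; A state machine advances a normalized time on Tick, driving the material's BlendPPEffect parameter and the curve-remapped post-process blend weight.
; It lazily spawns BP_VFX_ScanActor with a dynamic material, and on full fade-out stops ticking and optionally destroys that actor.
; Grid cell size and range go to MPC_VFX_ScanEffect at BeginPlay.
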(event `self.ReceiveBeginPlay`
  (bind _asbp_npcharacter (cast `/Game/Features/NPCs/BP_NPCharacter` (`self.GetOwner`))
    (:`then`
      (set `self.Owner` _asbp_npcharacter)
      (`self.UpdateScanState` "NewEnumerator3" true)
      (`KismetMaterialLibrary.SetScalarParameterValue` "/Game/Vfx/ScanEffect/MPC_VFX_ScanEffect.MPC_VFX_ScanEffect" "GridCellSize" (`self.GridCellSize`))
      (`KismetMaterialLibrary.SetScalarParameterValue` "/Game/Vfx/ScanEffect/MPC_VFX_ScanEffect.MPC_VFX_ScanEffect" "Range" (`self.Range`)))
    (:`CastFailed`
      (`self.UpdateScanState` "NewEnumerator4" true))))

(event `self.ReceiveTick`
  (params (DeltaSeconds :type "Float (single-precision)"))
  (bind _owner (`self.Owner`))
  (`self.UpdateScanTime` DeltaSeconds)
  (switch `/Game/Vfx/ScanEffect/EBP_VFX_ScanState` (`self.GetScanState`)
    (:`NewEnumerator0`
      (`self.UpdateScanPPBlendWeight` :!label _label))
    (:`NewEnumerator1`
      _)
    (:`NewEnumerator2`
      (goto _label))
    (:`NewEnumerator3`
      _))
  (`/Engine/EditorBlueprintResources/StandardMacros.IsValid` _owner
    (:`Is Valid`
      (set `self.Location` (`Actor.K2_GetActorLocation` _owner)))))

(fn `DestroyPPActor`
  (bind _scanactor (`self.ScanActor`))
  (if (and (`KismetSystemLibrary.IsValid` _scanactor) (`self.bDestroyActor`))
    (`Actor.K2_DestroyActor` _scanactor)
    (set `self.ScanActor` null)))

(fn `EndScanEffect`
  (returns (bEnded :type Boolean))
  (switch `/Game/Vfx/ScanEffect/EBP_VFX_ScanState` (`self.GetScanState`)
    (:`NewEnumerator0`
      _)
    (:`NewEnumerator1`
      _)
    (:`NewEnumerator2`
      (return false))
    (:`NewEnumerator3`
      (return false))
    (:`NewEnumerator4`
      (return false)))
  (bind _bupdated (`self.UpdateScanState` "NewEnumerator2"))
  (return _bupdated))

(fn `GetScanPPActor`
  (returns (ScanActor :type "/Game/Vfx/ScanEffect/BP_VFX_ScanActor Object Reference"))
  (bind _scanactor (`self.ScanActor`))
  (bind _ppmaterial (`self.PPMaterial`))
  (bind _postprocess (`/Game/Vfx/ScanEffect/BP_VFX_ScanActor.PostProcess` (`self.ScanActor`)))
  (`/Engine/EditorBlueprintResources/StandardMacros.IsValid` _scanactor
    (:`Is Valid`
      (return _scanactor))
    (:`Is Not Valid`
      (bind _returnvalue (`|SpawnActorFromClass` "/Game/Vfx/ScanEffect/BP_VFX_ScanActor.BP_VFX_ScanActor_C" (`KismetMathLibrary.MakeTransform` (0.0 0.0 0.0)) "Undefined" "MultiplyWithRoot" null null null))
      (set `self.ScanActor` _returnvalue)
      (`|ExecutionSequence`
        (:`then_0`
          (`/Engine/EditorBlueprintResources/StandardMacros.IsValid` (`self.PPMD`)
            (:`Is Valid`
              _)
            (:`Is Not Valid`
              (`/Engine/EditorBlueprintResources/StandardMacros.IsValid` _ppmaterial
                (:`Is Valid`
                  (bind _returnvalue_2 (`KismetMaterialLibrary.CreateDynamicMaterialInstance` _ppmaterial))
                  (set `self.PPMD` _returnvalue_2)))))
          (`/Engine/EditorBlueprintResources/StandardMacros.IsValid` _postprocess
            (:`Is Valid`
              (setmembers `PostProcessSettings` :`StructRef` (`PostProcessComponent.Settings` _postprocess) :`WeightedBlendables` (make `WeightedBlendables` (`|MakeArray` (make `WeightedBlendable` 1.0 (`self.PPMD`))))))))
        (:`then_1`
          (return _scanactor))))))

(fn `GetScanState`
  (returns (State :type "/Game/Vfx/ScanEffect/EBP_VFX_ScanState Enum"))
  (return (`self.State`)))

(fn `StartScanEffect`
  (returns (bStarted :type Boolean))
  (switch `/Game/Vfx/ScanEffect/EBP_VFX_ScanState` (`self.GetScanState`)
    (:`NewEnumerator0`
      _)
    (:`NewEnumerator1`
      _)
    (:`NewEnumerator2`
      (bind _bupdated (`self.UpdateScanState` "NewEnumerator0" :!label _label))
      (return _bupdated))
    (:`NewEnumerator3`
      (goto _label))
    (:`NewEnumerator4`
      _))
  (return false))

(fn `UpdateScanPPBlendWeight`
  (locals (ThisTime :type "Float (single-precision)" :default 0.0))
  (bind _ppblendcurve (`self.PPBlendCurve`))
  (bind _scannormalizedtime (`self.ScanNormalizedTime`))
  (`/Engine/EditorBlueprintResources/StandardMacros.IsValid` _ppblendcurve
    (:`Is Valid`
      (set `local.ThisTime` (`CurveFloat.GetFloatValue` _ppblendcurve _scannormalizedtime)))
    (:`Is Not Valid`
      (set `local.ThisTime` _scannormalizedtime)))
  (bind _scanactor (`self.GetScanPPActor`))
  (`/Engine/EditorBlueprintResources/StandardMacros.IsValid` _scanactor
    (:`Is Valid`
      (bind _postprocess (`/Game/Vfx/ScanEffect/BP_VFX_ScanActor.PostProcess` _scanactor))
      (`/Engine/EditorBlueprintResources/StandardMacros.IsValid` _postprocess
        (:`Is Valid`
          (set `PostProcessComponent.BlendWeight` (`local.ThisTime`) _postprocess))))))

(fn `UpdateScanState`
  (params (State :type "/Game/Vfx/ScanEffect/EBP_VFX_ScanState Enum" :default "NewEnumerator0") (bForce :type Boolean))
  (returns (bUpdated :type Boolean))
  (if (or (`|EnumInequality` State (`self.State`)) bForce)
    (`|ExecutionSequence`
      (:`then_0`
        (switch `/Game/Vfx/ScanEffect/EBP_VFX_ScanState` (`self.State`) ; exit current state
          (:`NewEnumerator1`
            (set `self.bFadedIn` 0.0))
          (:`NewEnumerator3`
            (set `self.bFadedOut` 0.0)
            (`self.SetComponentTickEnabled` true))))
      (:`then_1`
        (bind _output_get (set `self.State` State))
        (switch `/Game/Vfx/ScanEffect/EBP_VFX_ScanState` _output_get ; enter new state
          (:`NewEnumerator1`
            (set `self.bFadedIn` 1.0)
            (`self.UpdateScanPPBlendWeight`))
          (:`NewEnumerator3`
            (set `self.bFadedOut` 1.0)
            (`self.UpdateScanPPBlendWeight`)
            (`self.SetComponentTickEnabled` false :!label _label)
            (`self.DestroyPPActor`))
          (:`NewEnumerator4`
            (goto _label))))
      (:`then_2`
        (return true)))
    (else
      (return false))))

(fn `UpdateScanTime`
  (params (DeltaTime :type "Float (double-precision)"))
  (returns (bUpdated :type Boolean))
  (bind _ppmd (`self.PPMD`))
  (`|ExecutionSequence`
    (:`then_0`
      (switch `/Game/Vfx/ScanEffect/EBP_VFX_ScanState` (`self.GetScanState`)
        (:`NewEnumerator0`
          (bind _output_get (set `self.ScanNormalizedTime` (+ (`self.ScanNormalizedTime`) (* (`local.DeltaTime`) (`self.FadeInSpeed`)))))
          (if (>= _output_get 1.0)
            (set `self.ScanNormalizedTime` 1.0)
            (`self.UpdateScanState` "NewEnumerator1")))
        (:`NewEnumerator2`
          (bind _output_get_2 (set `self.ScanNormalizedTime` (- (`self.ScanNormalizedTime`) (* (`local.DeltaTime`) (`self.FadeOutSpeed`)))))
          (if (<= _output_get_2 0.0)
            (set `self.ScanNormalizedTime` 0.0)
            (`self.UpdateScanState` "NewEnumerator3")))
        (:`NewEnumerator4`
          (return true)))
      (`/Engine/EditorBlueprintResources/StandardMacros.IsValid` _ppmd
        (:`Is Valid`
          (`MaterialInstanceDynamic.SetScalarParameterValue` _ppmd "BlendPPEffect" (`self.ScanNormalizedTime`)))))
    (:`then_1`
      (return true))))